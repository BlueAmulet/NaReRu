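; Lightning bolt actor that plays a single thunder strike with flashing light and distance-delayed sound, then destroys itself.
; On BeginPlay it starts Lightning1, flickers a directional light through timed visibility toggles, then hides the light and particle system.
; It prints the strike distance and sound delay in Japanese, waits Distance / 3400 seconds to mimic the speed of sound, then plays Lightning.
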(event `self.ReceiveBeginPlay`
  (bind _distance (`self.Distance`))
  (bind _directionallight (`self.DirectionalLight`))
  (bind _returnvalue (/ _distance 3400.0))
  (`AudioComponent.Play` (`self.Lightning1`) 0.0)
  (`SceneComponent.SetHiddenInGame` _directionallight true false)
  (`KismetSystemLibrary.Delay` 0.5)
  (`SceneComponent.SetHiddenInGame` _directionallight false false)
  (`KismetSystemLibrary.Delay` 0.25)
  (`SceneComponent.SetHiddenInGame` _directionallight true false)
  (`KismetSystemLibrary.Delay` 0.1)
  (`SceneComponent.SetHiddenInGame` _directionallight false false)
  (`KismetSystemLibrary.Delay` 0.1)
  (`SceneComponent.SetHiddenInGame` _directionallight true false)
  (`SceneComponent.SetHiddenInGame` (`self.ParticleSystem`) true false)
  (`KismetSystemLibrary.PrintString` (`KismetStringLibrary.Concat_StrStr` "落雷距離" (`KismetStringLibrary.Conv_DoubleToString` (/ _distance 10.0)) "m" "      " "音が聞こえるまで" (`KismetStringLibrary.Conv_DoubleToString` _returnvalue) "秒") true true (struct :`G` 0.190395 :`B` 1.0 :`A` 1.0) 10.0)
  (`KismetSystemLibrary.Delay` _returnvalue)
  (`AudioComponent.Play` (`self.Lightning`) 0.0)
  (`KismetSystemLibrary.Delay` 10.0)
  (`self.K2_DestroyActor`))

(fn `UserConstructionScript`)