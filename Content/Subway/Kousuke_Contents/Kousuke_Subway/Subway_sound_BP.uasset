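; Subway train sound Blueprint that plays door, departure, running, arrival and emergency-stop audio through CRI cues.
; Departure, arrival and emergency-stop events time cue starts with delays and ramp AISAC controls to fade between VVVF, running and arriving sounds.
; Three Delay-based loop macros drive these ramps every 0.1 seconds until CrossFade or CrossFadeArriving reaches its limit.
; The emergency stop follows its fade with a delayed safety-check sound.
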(event `Play_Subway_door_close`
  (`AtomComponent.Play` (`self.Train_door_close1`) 0.0)
  (`AtomComponent.Play` (`self.Subway_door_close`) 0.0))

(event `Play_Subway_door_open`
  (`AtomComponent.Play` (`self.Train_door_open1`) 0.0))

(event `tokyo_arrive`
  (`AtomComponent.Play` (`self.Train_door_close_Tokyo`) 0.0))

(event `Play_Subway_syuppatsu`
  (`|ExecutionSequence`
    (:`then_0`
      (`KismetSystemLibrary.Delay` 40.0)
      (`self.Loop_delay`
        (:`Loop`
          (bind _output_get (set `self.CrossFade` (+ (`self.CrossFade`) 0.01)))
          (`AtomComponent.SetAisacByName` (`self.Subway_VVVF_runnning_loop_cue`) "AisacControl_00" _output_get))))
    (:`then_1`
      (`KismetSystemLibrary.Delay` 0.2)
      (`AtomComponent.Play` (`self.Subway_VVVF_runnning_loop_cue`) 0.0)
      (`KismetSystemLibrary.Delay` 21.0)
      (`AtomComponent.Play` (`self.Subway_run_loop_cue`) 0.0))
    (:`then_2`
      (`KismetSystemLibrary.Delay` 40.0)
      (`self.Loop_delay`
        (:`Loop`
          (bind _output_get_2 (set `self.CrossFade` (+ (`self.CrossFade`) 0.01)))
          (`AtomComponent.SetAisacByName` (`self.Subway_run_loop_cue`) "AisacControl_00" _output_get_2))
        (:`End`
          (`AtomComponent.Stop` (`self.Subway_VVVF_runnning_loop_cue`))
          (`AtomComponent.SetAisacByName` (`self.Subway_VVVF_runnning_loop_cue`) "AisacControl_00" 0.0)
          (`AtomComponent.SetAisacByName` (`self.Subway_arriving_cue`) "AisacControl_02" 0.0))))
    (:`then_3`
      (`AtomComponent.SetAisacByName` (`self.Subway_run_loop_cue`) "AisacControl_00" 1.0))))

(event `Subway_set_Aisac_toutyaku`
  (`|ExecutionSequence`
    (:`then_0`
      (`KismetSystemLibrary.Delay` 20.0)
      (`self.Loop_delay_crossfade_running`
        (:`Loop`
          (bind _output_get (set `self.CrossFade` (+ (`self.CrossFade`) -0.03 0.0)))
          (`AtomComponent.SetAisacByName` (`self.Subway_run_loop_cue`) "AisacControl_00" _output_get))
        (:`End`
          (`AtomComponent.Stop` (`self.Subway_run_loop_cue`)))))
    (:`then_1`
      (`KismetSystemLibrary.Delay` 14.0)
      (`AtomComponent.Play` (`self.Subway_arriving_cue`) 0.0)
      (`self.Loop_delay_crossfade_arriving`
        (:`Loop`
          (bind _output_get_2 (set `self.CrossFade_arriving` (+ (`self.CrossFade_arriving`) 0.3)))
          (`AtomComponent.SetAisacByName` (`self.Subway_arriving_cue`) "AisacControl_02" _output_get_2))))))

(event `急停車音`
  (`AtomComponent.Play` (`self.Subway_arriving_cue`) 3.0)
  (`self.Loop_delay_crossfade_arriving`
    (:`Loop`
      (bind _output_get (set `self.CrossFade_arriving` (+ (`self.CrossFade_arriving`) 0.1)))
      (`AtomComponent.SetAisacByName` (`self.Subway_arriving_cue`) "AisacControl_02" _output_get))
    (:`End`
      (`KismetSystemLibrary.Delay` 10.0)
      (`AtomComponent.Play` (`self.安全確認`) 0.0))))

(fn `UserConstructionScript`)