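; Subway announcement Blueprint that plays in-train station audio for stops from Shinotsuka through Tokyo, plus a standalone "omatase" clip.
; Each station has its own event that plays a "Next" audio clip after a short delay, then a "Soon" arrival clip after a longer fixed delay.
; Timing is hard-coded and identical for every stop except Tokyo, which waits longer before its arrival clip.
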(event `Play_omatase`
  (`AtomComponent.Play` (`self.omatase`) 0.0))

(event `Play_announce_shinotsuka`
  (`KismetSystemLibrary.Delay` 10.0)
  (`AtomComponent.Play` (`self.Next_shinotsuka`) 0.0)
  (`KismetSystemLibrary.Delay` 130.0)
  (`AtomComponent.Play` (`self.Soon_shinotsuka`) 0.0))

(event `Play_announce_myogadani`
  (`KismetSystemLibrary.Delay` 10.0)
  (`AtomComponent.Play` (`self.Next_myogadani`) 0.0)
  (`KismetSystemLibrary.Delay` 130.0)
  (`AtomComponent.Play` (`self.Soon_myogadani`) 0.0))

(event `Play_announce_korakuen`
  (`KismetSystemLibrary.Delay` 10.0)
  (`AtomComponent.Play` (`self.Next_korakuen`) 0.0)
  (`KismetSystemLibrary.Delay` 130.0)
  (`AtomComponent.Play` (`self.Soon_korakuen`) 0.0))

(event `Play_announce_hongosanchome`
  (`KismetSystemLibrary.Delay` 10.0)
  (`AtomComponent.Play` (`self.Next_hongosanchome`) 0.0)
  (`KismetSystemLibrary.Delay` 130.0)
  (`AtomComponent.Play` (`self.Soon_hongosanchome`) 0.0))

(event `Play_announce_ochanomizu`
  (`KismetSystemLibrary.Delay` 10.0)
  (`AtomComponent.Play` (`self.Next_ochanomizu`) 0.0)
  (`KismetSystemLibrary.Delay` 130.0)
  (`AtomComponent.Play` (`self.Soon_ochanomizu`) 0.0))

(event `Play_announce_awajicho`
  (`KismetSystemLibrary.Delay` 10.0)
  (`AtomComponent.Play` (`self.Next_awajicho`) 0.0)
  (`KismetSystemLibrary.Delay` 130.0)
  (`AtomComponent.Play` (`self.Soon_awajicho`) 0.0))

(event `Play_announce_otemachi`
  (`KismetSystemLibrary.Delay` 10.0)
  (`AtomComponent.Play` (`self.Next_otemachi`) 0.0)
  (`KismetSystemLibrary.Delay` 130.0)
  (`AtomComponent.Play` (`self.Soon_otemachi`) 0.0))

(event `Play_announce_tokyo`
  (`KismetSystemLibrary.Delay` 10.0)
  (`AtomComponent.Play` (`self.Next_tokyo`) 0.0)
  (`KismetSystemLibrary.Delay` 165.0)
  (`AtomComponent.Play` (`self.Soon_tokyo`) 0.0))

(fn `UserConstructionScript`)