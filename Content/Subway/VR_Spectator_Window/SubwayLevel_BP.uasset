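; SubwayLevel_BP runs a VR subway ride from Ikebukuro to Tokyo, one event and timeline per segment.
; Timelines slide station actors past the train, update SubwayWindow progress, cue arrival audio and, except the last, swap streamed levels.
; A FlipFlop emergency stop animates 急停車_BP and pauses or resumes the timeline matching the widget's StationNum.
; Boarding and alighting events move the VR player by timeline, with alighting also raising camera height.
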(event `池袋to新大塚`
  ;[1 1 1] 池袋から新大塚まで
  (bind (_direction `_電車_駅_の動き` `_インジケーター`) (`Timeline|タイムライン_電車の動き` :!label _label)
    (:`Update`
      (bind _returnvalue (`GameplayStatics.GetActorOfClass` "/Game/Subway/Marks_Contents/OBJ/station/Station_BP/Ikebukuro_BP.Ikebukuro_BP_C"))
      (`self.K2_SetActorRelativeLocation` _returnvalue (`KismetMathLibrary.MakeVector` 0.0 `_電車_駅_の動き`) false false)
      (bind _returnvalue_2 (`GameplayStatics.GetActorOfClass` "/Game/Subway/Marks_Contents/OBJ/station/Station_BP/sinotsuka_BP.sinotsuka_BP_C"))
      (`self.K2_SetActorLocation` _returnvalue_2 (`KismetMathLibrary.MakeVector` 0.0 (+ `_電車_駅_の動き` 200000.0)) false false)
      (bind _foundwidgets (`WidgetBlueprintLibrary.GetAllWidgetsOfClass` "/Game/Subway/VR_Spectator_Window/SubwayWindow.SubwayWindow_C" false))
      (for _array_element _foundwidgets
        (set `/Game/Subway/VR_Spectator_Window/SubwayWindow.Subway_Percentage` `_インジケーター` _array_element)))
    (:`Finished`
      ;;[1 1 1] レベル移行
      (`KismetSystemLibrary.Delay` 2.0)
      (`GameplayStatics.LoadStreamLevel` "2shinotuka_myougadani" true)
      (`GameplayStatics.UnloadStreamLevel` "1Ikebukuro_shinotuka")
      (bind _foundwidgets_2 (`WidgetBlueprintLibrary.GetAllWidgetsOfClass` "/Game/Subway/VR_Spectator_Window/SubwayWindow.SubwayWindow_C" false))
      (`/Game/Subway/VR_Spectator_Window/SubwayWindow.ボタンON` _foundwidgets_2))
    (:`駅出現`
      (bind _returnvalue_3 (`GameplayStatics.GetActorOfClass` "/Game/Subway/Kousuke_Contents/Kousuke_Subway/Subway_sound_BP.Subway_sound_BP_C"))
      (`/Game/Subway/Kousuke_Contents/Kousuke_Subway/Subway_sound_BP.Subway_set_Aisac_toutyaku` _returnvalue_3))
    (:`急停車ボタン`
      (bind _foundwidgets_3 (`WidgetBlueprintLibrary.GetAllWidgetsOfClass` "/Game/Subway/VR_Spectator_Window/SubwayWindow.SubwayWindow_C" false))
      (`/Game/Subway/VR_Spectator_Window/SubwayWindow.急停車ボタン` _foundwidgets_3))))

(event `新大塚to茗荷谷`
  ;[1 1 1] 新大塚から茗荷谷まで
  (bind (_direction `_電車_駅_の動き` `_インジケーター`) (`Timeline|タイムライン_1` :!label _label_2)
    (:`Update`
      (`|ExecutionSequence`
        (:`then_0`
          (bind _outactors (`GameplayStatics.GetAllActorsOfClass` "/Game/Subway/Marks_Contents/OBJ/station/Station_BP/sinotsuka_BP.sinotsuka_BP_C"))
          (`self.K2_SetActorRelativeLocation` _outactors (`KismetMathLibrary.MakeVector` 0.0 `_電車_駅_の動き`) false false)
          (bind _foundwidgets (`WidgetBlueprintLibrary.GetAllWidgetsOfClass` "/Game/Subway/VR_Spectator_Window/SubwayWindow.SubwayWindow_C" false))
          (for _array_element _foundwidgets
            (set `/Game/Subway/VR_Spectator_Window/SubwayWindow.Subway_Percentage` `_インジケーター` _array_element)))
        (:`then_1`
          (bind _outactors_2 (`GameplayStatics.GetAllActorsOfClass` "/Game/Subway/Marks_Contents/OBJ/station/Station_BP/Myogadani_BP.Myogadani_BP_C"))
          (for _array_element_2 _outactors_2
            (`self.K2_SetActorLocation` _array_element_2 (`KismetMathLibrary.MakeVector` 0.0 (+ `_電車_駅_の動き` 200000.0)) false false)))))
    (:`Finished`
      ;;[1 1 1] レベル移動
      (`GameplayStatics.LoadStreamLevel` "3myougadani_kourakuen" true)
      (`GameplayStatics.UnloadStreamLevel` "2shinotuka_myougadani")
      (bind _foundwidgets_2 (`WidgetBlueprintLibrary.GetAllWidgetsOfClass` "/Game/Subway/VR_Spectator_Window/SubwayWindow.SubwayWindow_C" false))
      (`/Game/Subway/VR_Spectator_Window/SubwayWindow.ボタンON` _foundwidgets_2))
    (:`駅出現`
      (bind _returnvalue (`GameplayStatics.GetActorOfClass` "/Game/Subway/Kousuke_Contents/Kousuke_Subway/Subway_sound_BP.Subway_sound_BP_C"))
      (`/Game/Subway/Kousuke_Contents/Kousuke_Subway/Subway_sound_BP.Subway_set_Aisac_toutyaku` _returnvalue))
    (:`急停車ボタン`
      (bind _foundwidgets_3 (`WidgetBlueprintLibrary.GetAllWidgetsOfClass` "/Game/Subway/VR_Spectator_Window/SubwayWindow.SubwayWindow_C" false))
      (`/Game/Subway/VR_Spectator_Window/SubwayWindow.急停車ボタン` _foundwidgets_3))))

(event `self.ReceiveBeginPlay`
  (bind _returnvalue (`GameplayStatics.GetActorOfClass` "/Game/Subway/Blueprint/急停車_BP.急停車_BP_C"))
  (`self.SetActorHiddenInGame` _returnvalue true))

(event `カスタムイベント_急停車`
  (`/Engine/EditorBlueprintResources/StandardMacros.FlipFlop`
    (:`A`
      (`KismetSystemLibrary.PrintString` "急停車")
      (`AtomComponent.Play` (`self.Atom＿急停車`) 0.0)
      (bind _returnvalue (`GameplayStatics.GetActorOfClass` "/Game/Subway/Blueprint/急停車_BP.急停車_BP_C"))
      (`self.SetActorHiddenInGame` _returnvalue false)
      (bind (_direction `_新規track_0`) (`Timeline|急停車` :!via `PlayFromStart`)
        (:`Update`
          (`self.K2_SetActorRelativeLocation` _returnvalue `_新規track_0` false false))
        (:`駅BP停止`
          (bind _foundwidgets (`WidgetBlueprintLibrary.GetAllWidgetsOfClass` "/Game/Subway/VR_Spectator_Window/SubwayWindow.SubwayWindow_C" false))
          (for _array_element _foundwidgets
            (switch `int` (`/Game/Subway/VR_Spectator_Window/SubwayWindow.StationNum` _array_element)
              (:`0`
                (goto _label :!via `Stop`))
              (:`1`
                (goto _label_2 :!via `Stop`))
              (:`2`
                ;[1 1 1] 茗荷谷から後楽園まで
                (bind (_direction_2 `_電車_駅_の動き` `_インジケーター`) (`Timeline|タイムライン_2` :!via `Stop` :!label _label_3)
                  (:`Update`
                    (`|ExecutionSequence`
                      (:`then_0`
                        (bind _outactors (`GameplayStatics.GetAllActorsOfClass` "/Game/Subway/Marks_Contents/OBJ/station/Station_BP/Myogadani_BP.Myogadani_BP_C"))
                        (`self.K2_SetActorRelativeLocation` _outactors (`KismetMathLibrary.MakeVector` 0.0 `_電車_駅_の動き`) false false)
                        (bind _foundwidgets_2 (`WidgetBlueprintLibrary.GetAllWidgetsOfClass` "/Game/Subway/VR_Spectator_Window/SubwayWindow.SubwayWindow_C" false))
                        (for _array_element_2 _foundwidgets_2
                          (set `/Game/Subway/VR_Spectator_Window/SubwayWindow.Subway_Percentage` `_インジケーター` _array_element_2)))
                      (:`then_1`
                        (bind _outactors_2 (`GameplayStatics.GetAllActorsOfClass` "/Game/Subway/Marks_Contents/OBJ/station/Station_BP/Korakuen_BP.Korakuen_BP_C"))
                        (for _array_element_3 _outactors_2
                          (`self.K2_SetActorLocation` _array_element_3 (`KismetMathLibrary.MakeVector` 0.0 (+ `_電車_駅_の動き` 200000.0)) false false)))))
                  (:`Finished`
                    ;;[1 1 1] レベル移動
                    (`KismetSystemLibrary.Delay` 2.0)
                    (`GameplayStatics.LoadStreamLevel` "4kourakuen_hongou" true)
                    (`GameplayStatics.UnloadStreamLevel` "3myougadani_kourakuen")
                    (bind _foundwidgets_3 (`WidgetBlueprintLibrary.GetAllWidgetsOfClass` "/Game/Subway/VR_Spectator_Window/SubwayWindow.SubwayWindow_C" false))
                    (`/Game/Subway/VR_Spectator_Window/SubwayWindow.ボタンON` _foundwidgets_3))
                  (:`駅出現`
                    (bind _returnvalue_2 (`GameplayStatics.GetActorOfClass` "/Game/Subway/Kousuke_Contents/Kousuke_Subway/Subway_sound_BP.Subway_sound_BP_C"))
                    (`/Game/Subway/Kousuke_Contents/Kousuke_Subway/Subway_sound_BP.Subway_set_Aisac_toutyaku` _returnvalue_2))
                  (:`急停車ボタン`
                    (bind _foundwidgets_4 (`WidgetBlueprintLibrary.GetAllWidgetsOfClass` "/Game/Subway/VR_Spectator_Window/SubwayWindow.SubwayWindow_C" false))
                    (`/Game/Subway/VR_Spectator_Window/SubwayWindow.急停車ボタン` _foundwidgets_4))))
              (:`3`
                ;[1 1 1] 後楽園から本郷まで
                (bind (_direction_3 `_電車_駅_の動き_2` `_インジケーター_2`) (`Timeline|タイムライン_3` :!via `Stop` :!label _label_4)
                  (:`Update`
                    (`|ExecutionSequence`
                      (:`then_0`
                        (bind _outactors_3 (`GameplayStatics.GetAllActorsOfClass` "/Game/Subway/Marks_Contents/OBJ/station/Station_BP/Korakuen_BP.Korakuen_BP_C"))
                        (`self.K2_SetActorRelativeLocation` _outactors_3 (`KismetMathLibrary.MakeVector` 0.0 `_電車_駅_の動き_2`) false false)
                        (bind _foundwidgets_5 (`WidgetBlueprintLibrary.GetAllWidgetsOfClass` "/Game/Subway/VR_Spectator_Window/SubwayWindow.SubwayWindow_C" false))
                        (for _array_element_4 _foundwidgets_5
                          (set `/Game/Subway/VR_Spectator_Window/SubwayWindow.Subway_Percentage` `_インジケーター_2` _array_element_4)))
                      (:`then_1`
                        (bind _outactors_4 (`GameplayStatics.GetAllActorsOfClass` "/Game/Subway/Marks_Contents/OBJ/station/Station_BP/honhongousanchoume_BP.honhongousanchoume_BP_C"))
                        (for _array_element_5 _outactors_4
                          (`self.K2_SetActorLocation` _array_element_5 (`KismetMathLibrary.MakeVector` 0.0 (+ `_電車_駅_の動き_2` 200000.0)) false false)))))
                  (:`Finished`
                    ;;[1 1 1] レベル移動
                    (`KismetSystemLibrary.Delay` 2.0)
                    (`GameplayStatics.LoadStreamLevel` "5hongou_ochanomizu" true)
                    (`GameplayStatics.UnloadStreamLevel` "4kourakuen_hongou")
                    (bind _foundwidgets_6 (`WidgetBlueprintLibrary.GetAllWidgetsOfClass` "/Game/Subway/VR_Spectator_Window/SubwayWindow.SubwayWindow_C" false))
                    (`/Game/Subway/VR_Spectator_Window/SubwayWindow.ボタンON` _foundwidgets_6))
                  (:`駅出現`
                    (bind _returnvalue_3 (`GameplayStatics.GetActorOfClass` "/Game/Subway/Kousuke_Contents/Kousuke_Subway/Subway_sound_BP.Subway_sound_BP_C"))
                    (`/Game/Subway/Kousuke_Contents/Kousuke_Subway/Subway_sound_BP.Subway_set_Aisac_toutyaku` _returnvalue_3))
                  (:`急停車ボタン`
                    (bind _foundwidgets_7 (`WidgetBlueprintLibrary.GetAllWidgetsOfClass` "/Game/Subway/VR_Spectator_Window/SubwayWindow.SubwayWindow_C" false))
                    (`/Game/Subway/VR_Spectator_Window/SubwayWindow.急停車ボタン` _foundwidgets_7))))
              (:`4`
                ;[1 1 1] 本郷から御茶ノ水
                (bind (_direction_4 `_電車_駅_の動き_3` `_インジケーター_3`) (`Timeline|タイムライン_4` :!via `Stop` :!label _label_5)
                  (:`Update`
                    (`|ExecutionSequence`
                      (:`then_0`
                        (bind _outactors_5 (`GameplayStatics.GetAllActorsOfClass` "/Game/Subway/Marks_Contents/OBJ/station/Station_BP/honhongousanchoume_BP.honhongousanchoume_BP_C"))
                        (`self.K2_SetActorRelativeLocation` _outactors_5 (`KismetMathLibrary.MakeVector` 0.0 `_電車_駅_の動き_3`) false false)
                        (bind _foundwidgets_8 (`WidgetBlueprintLibrary.GetAllWidgetsOfClass` "/Game/Subway/VR_Spectator_Window/SubwayWindow.SubwayWindow_C" false))
                        (for _array_element_6 _foundwidgets_8
                          (set `/Game/Subway/VR_Spectator_Window/SubwayWindow.Subway_Percentage` `_インジケーター_3` _array_element_6)))
                      (:`then_1`
                        (bind _outactors_6 (`GameplayStatics.GetAllActorsOfClass` "/Game/Subway/Marks_Contents/OBJ/station/Station_BP/Ochanomizu_BP.Ochanomizu_BP_C"))
                        (for _array_element_7 _outactors_6
                          (`self.K2_SetActorLocation` _array_element_7 (`KismetMathLibrary.MakeVector` 0.0 (+ `_電車_駅_の動き_3` 200000.0)) false false)))))
                  (:`Finished`
                    ;;[1 1 1] レベル移動
                    (`KismetSystemLibrary.Delay` 2.0)
                    (`GameplayStatics.LoadStreamLevel` "6ochanomizu_awajichou" true)
                    (`GameplayStatics.UnloadStreamLevel` "5hongou_ochanomizu")
                    (bind _foundwidgets_9 (`WidgetBlueprintLibrary.GetAllWidgetsOfClass` "/Game/Subway/VR_Spectator_Window/SubwayWindow.SubwayWindow_C" false))
                    (`/Game/Subway/VR_Spectator_Window/SubwayWindow.ボタンON` _foundwidgets_9))
                  (:`駅出現`
                    (bind _returnvalue_4 (`GameplayStatics.GetActorOfClass` "/Game/Subway/Kousuke_Contents/Kousuke_Subway/Subway_sound_BP.Subway_sound_BP_C"))
                    (`/Game/Subway/Kousuke_Contents/Kousuke_Subway/Subway_sound_BP.Subway_set_Aisac_toutyaku` _returnvalue_4))
                  (:`急停車ボタン`
                    (bind _foundwidgets_10 (`WidgetBlueprintLibrary.GetAllWidgetsOfClass` "/Game/Subway/VR_Spectator_Window/SubwayWindow.SubwayWindow_C" false))
                    (`/Game/Subway/VR_Spectator_Window/SubwayWindow.急停車ボタン` _foundwidgets_10))))
              (:`5`
                ;[1 1 1] 御茶ノ水から淡路町まで
                (bind (_direction_5 `_電車_駅_の動き_4` `_インジケーター_4`) (`Timeline|タイムライン_5` :!via `Stop` :!label _label_6)
                  (:`Update`
                    (`|ExecutionSequence`
                      (:`then_0`
                        (bind _outactors_7 (`GameplayStatics.GetAllActorsOfClass` "/Game/Subway/Marks_Contents/OBJ/station/Station_BP/Ochanomizu_BP.Ochanomizu_BP_C"))
                        (`self.K2_SetActorRelativeLocation` _outactors_7 (`KismetMathLibrary.MakeVector` 0.0 `_電車_駅_の動き_4`) false false)
                        (bind _foundwidgets_11 (`WidgetBlueprintLibrary.GetAllWidgetsOfClass` "/Game/Subway/VR_Spectator_Window/SubwayWindow.SubwayWindow_C" false))
                        (for _array_element_8 _foundwidgets_11
                          (set `/Game/Subway/VR_Spectator_Window/SubwayWindow.Subway_Percentage` `_インジケーター_4` _array_element_8)))
                      (:`then_1`
                        (bind _outactors_8 (`GameplayStatics.GetAllActorsOfClass` "/Game/Subway/Marks_Contents/OBJ/station/Station_BP/Awajicho_BP.Awajicho_BP_C"))
                        (for _array_element_9 _outactors_8
                          (`self.K2_SetActorLocation` _array_element_9 (`KismetMathLibrary.MakeVector` 0.0 (+ `_電車_駅_の動き_4` 200000.0)) false false)))))
                  (:`Finished`
                    ;;[1 1 1] レベル移動
                    (`KismetSystemLibrary.Delay` 2.0)
                    (`GameplayStatics.LoadStreamLevel` "7awajichou_otemachi" true)
                    (`GameplayStatics.UnloadStreamLevel` "6ochanomizu_awajichou")
                    (bind _foundwidgets_12 (`WidgetBlueprintLibrary.GetAllWidgetsOfClass` "/Game/Subway/VR_Spectator_Window/SubwayWindow.SubwayWindow_C" false))
                    (`/Game/Subway/VR_Spectator_Window/SubwayWindow.ボタンON` _foundwidgets_12))
                  (:`駅出現`
                    (bind _returnvalue_5 (`GameplayStatics.GetActorOfClass` "/Game/Subway/Kousuke_Contents/Kousuke_Subway/Subway_sound_BP.Subway_sound_BP_C"))
                    (`/Game/Subway/Kousuke_Contents/Kousuke_Subway/Subway_sound_BP.Subway_set_Aisac_toutyaku` _returnvalue_5))
                  (:`急停車ボタン`
                    (bind _foundwidgets_13 (`WidgetBlueprintLibrary.GetAllWidgetsOfClass` "/Game/Subway/VR_Spectator_Window/SubwayWindow.SubwayWindow_C" false))
                    (`/Game/Subway/VR_Spectator_Window/SubwayWindow.急停車ボタン` _foundwidgets_13))))
              (:`6`
                ;[1 1 1] 淡路町から大手町
                (bind (_direction_6 `_電車_駅_の動き_5` `_インジケーター_5`) (`Timeline|タイムライン_6` :!via `Stop` :!label _label_7)
                  (:`Update`
                    (`|ExecutionSequence`
                      (:`then_0`
                        (bind _outactors_9 (`GameplayStatics.GetAllActorsOfClass` "/Game/Subway/Marks_Contents/OBJ/station/Station_BP/Awajicho_BP.Awajicho_BP_C"))
                        (`self.K2_SetActorRelativeLocation` _outactors_9 (`KismetMathLibrary.MakeVector` 0.0 `_電車_駅_の動き_5`) false false)
                        (bind _foundwidgets_14 (`WidgetBlueprintLibrary.GetAllWidgetsOfClass` "/Game/Subway/VR_Spectator_Window/SubwayWindow.SubwayWindow_C" false))
                        (for _array_element_10 _foundwidgets_14
                          (set `/Game/Subway/VR_Spectator_Window/SubwayWindow.Subway_Percentage` `_インジケーター_5` _array_element_10)))
                      (:`then_1`
                        (bind _outactors_10 (`GameplayStatics.GetAllActorsOfClass` "/Game/Subway/Marks_Contents/OBJ/station/Station_BP/Otemachi_BP.Otemachi_BP_C"))
                        (for _array_element_11 _outactors_10
                          (`self.K2_SetActorLocation` _array_element_11 (`KismetMathLibrary.MakeVector` 0.0 (+ `_電車_駅_の動き_5` 200000.0)) false false)))))
                  (:`Finished`
                    ;;[1 1 1] レベル移動
                    (`KismetSystemLibrary.Delay` 2.0)
                    (`GameplayStatics.LoadStreamLevel` "8otemachi_tokyo" true)
                    (`GameplayStatics.UnloadStreamLevel` "7awajichou_otemachi")
                    (bind _foundwidgets_15 (`WidgetBlueprintLibrary.GetAllWidgetsOfClass` "/Game/Subway/VR_Spectator_Window/SubwayWindow.SubwayWindow_C" false))
                    (`/Game/Subway/VR_Spectator_Window/SubwayWindow.ボタンON` _foundwidgets_15))
                  (:`駅出現`
                    (bind _returnvalue_6 (`GameplayStatics.GetActorOfClass` "/Game/Subway/Kousuke_Contents/Kousuke_Subway/Subway_sound_BP.Subway_sound_BP_C"))
                    (`/Game/Subway/Kousuke_Contents/Kousuke_Subway/Subway_sound_BP.Subway_set_Aisac_toutyaku` _returnvalue_6))
                  (:`急停車ボタン`
                    (bind _foundwidgets_16 (`WidgetBlueprintLibrary.GetAllWidgetsOfClass` "/Game/Subway/VR_Spectator_Window/SubwayWindow.SubwayWindow_C" false))
                    (`/Game/Subway/VR_Spectator_Window/SubwayWindow.急停車ボタン` _foundwidgets_16))))
              (:`7`
                ;[1 1 1] 淡路町から大手町
                (bind (_direction_7 `_電車_駅_の動き_6` `_新規track_0_2`) (`Timeline|タイムライン_7` :!via `Stop` :!label _label_8)
                  (:`Update`
                    (`|ExecutionSequence`
                      (:`then_0`
                        (bind _outactors_11 (`GameplayStatics.GetAllActorsOfClass` "/Game/Subway/Marks_Contents/OBJ/station/Station_BP/Otemachi_BP.Otemachi_BP_C"))
                        (`self.K2_SetActorRelativeLocation` _outactors_11 (`KismetMathLibrary.MakeVector` 0.0 `_電車_駅_の動き_6`) false false)
                        (bind _foundwidgets_17 (`WidgetBlueprintLibrary.GetAllWidgetsOfClass` "/Game/Subway/VR_Spectator_Window/SubwayWindow.SubwayWindow_C" false))
                        (for _array_element_12 _foundwidgets_17
                          (set `/Game/Subway/VR_Spectator_Window/SubwayWindow.Subway_Percentage` `_新規track_0_2` _array_element_12)))
                      (:`then_1`
                        (bind _outactors_12 (`GameplayStatics.GetAllActorsOfClass` "/Game/Subway/Marks_Contents/OBJ/station/Station_BP/Tokyo_BP.Tokyo_BP_C"))
                        (for _array_element_13 _outactors_12
                          (`self.K2_SetActorLocation` _array_element_13 (`KismetMathLibrary.MakeVector` 0.0 (+ `_電車_駅_の動き_6` 200000.0)) false false)))))
                  (:`駅出現`
                    (bind _returnvalue_7 (`GameplayStatics.GetActorOfClass` "/Game/Subway/Kousuke_Contents/Kousuke_Subway/Subway_sound_BP.Subway_sound_BP_C"))
                    (`/Game/Subway/Kousuke_Contents/Kousuke_Subway/Subway_sound_BP.Subway_set_Aisac_toutyaku` _returnvalue_7))
                  (:`急停車ボタン`
                    (bind _foundwidgets_18 (`WidgetBlueprintLibrary.GetAllWidgetsOfClass` "/Game/Subway/VR_Spectator_Window/SubwayWindow.SubwayWindow_C" false))
                    (`/Game/Subway/VR_Spectator_Window/SubwayWindow.急停車ボタン` _foundwidgets_18)))))))))
    (:`B`
      (`|ExecutionSequence`
        (:`then_0`
          (bind _foundwidgets_19 (`WidgetBlueprintLibrary.GetAllWidgetsOfClass` "/Game/Subway/VR_Spectator_Window/SubwayWindow.SubwayWindow_C" false))
          (for _array_element_14 _foundwidgets_19
            (switch `int` (`/Game/Subway/VR_Spectator_Window/SubwayWindow.StationNum` _array_element_14)
              (:`0`
                (goto _label))
              (:`1`
                (goto _label_2))
              (:`2`
                (goto _label_3))
              (:`3`
                (goto _label_4))
              (:`4`
                (goto _label_5))
              (:`5`
                (goto _label_6))
              (:`6`
                (goto _label_7))
              (:`7`
                (goto _label_8)))))
        (:`then_1`
          (bind (_direction_8 `_トンネル移動`) (`Timeline|タイムライン_9` :!via `PlayFromStart`)
            (:`Update`
              (`self.K2_SetActorRelativeLocation` _returnvalue `_トンネル移動` false false))
            (:`Finished`
              (`self.SetActorHiddenInGame` _returnvalue true))))))))

(event `茗荷谷to後楽園`
  ;[1 1 1] 茗荷谷から後楽園まで
  (goto _label_3))

(event `乗車`
  ;[1 1 1] プレイヤー下車
  (`self.乗車_R`)
  (bind _outactors (`GameplayStatics.GetAllActorsOfClass` "SubwayLevel_BP_C"))
  (add `self.乗車_L` _outactors (delegate `乗車_左`)))

(event `乗車_左`
  ;[1 1 1] プレイヤー下車
  (bind (_direction `_プレイヤー移動`) (`Timeline|タイムライン_8` :!via `PlayFromStart` :!label _label_9)
    (:`Update`
      (bind _returnvalue (`GameplayStatics.GetActorOfClass` "/Game/NaReRu_Common/VR_Character/VRPlayer_Character.VRPlayer_Character_C"))
      (`self.K2_SetActorLocationAndRotation` _returnvalue (`KismetMathLibrary.MakeVector` (.x `_プレイヤー移動`) (.y `_プレイヤー移動`) (.z (`self.K2_GetActorLocation` (`GameplayStatics.GetPlayerCharacter` 0)))) (`KismetMathLibrary.MakeRotator` 0.0) true false))))

(event `下車_左`
  ;[1 1 1] プレイヤー下車
  (`KismetSystemLibrary.PrintString` "下車")
  (bind _returnvalue (`GameplayStatics.GetActorOfClass` "/Game/NaReRu_Common/VR_Character/VRPlayer_Character.VRPlayer_Character_C"))
  (set `/Game/NaReRu_Common/VR_Character/VRPlayer_Character.VRCameraHight` (+ (`/Game/NaReRu_Common/VR_Character/VRPlayer_Character.VRCameraHight` _returnvalue) 25.0) _returnvalue)
  (`/Game/NaReRu_Common/VR_Character/VRPlayer_Character.身長変更` _returnvalue)
  (goto _label_9 :!via `ReverseFromEnd`))

(event `後楽園to本郷`
  ;[1 1 1] 後楽園から本郷まで
  (goto _label_4))

(event `本郷to御茶ノ水`
  ;[1 1 1] 本郷から御茶ノ水
  (goto _label_5))

(event `御茶ノ水to淡路町`
  ;[1 1 1] 御茶ノ水から淡路町まで
  (goto _label_6))

(event `淡路町to大手町`
  ;[1 1 1] 淡路町から大手町
  (goto _label_7))

(event `大手町to東京`
  ;[1 1 1] 淡路町から大手町
  (goto _label_8))

(event `下車_L`
  (bind _returnvalue (`GameplayStatics.GetActorOfClass` "/Game/NaReRu_Common/VR_Character/VRPlayer_Character.VRPlayer_Character_C"))
  ;[1 1 1] 淡路町から大手町
  (set `/Game/NaReRu_Common/VR_Character/VRPlayer_Character.VRCameraHight` (+ (`/Game/NaReRu_Common/VR_Character/VRPlayer_Character.VRCameraHight` _returnvalue) 40.0) _returnvalue)
  (`/Game/NaReRu_Common/VR_Character/VRPlayer_Character.身長変更` _returnvalue)
  (bind (_direction `_移動` `_ローテーション`) (`Timeline|タイムライン_0` :!via `ReverseFromEnd`)
    (:`Update`
      (bind _returnvalue_2 (`GameplayStatics.GetActorOfClass` "/Game/NaReRu_Common/VR_Character/VRPlayer_Character.VRPlayer_Character_C"))
      (`self.K2_SetActorLocationAndRotation` _returnvalue_2 (`KismetMathLibrary.MakeVector` (.x `_移動`) (.y `_移動`) (.z (`self.K2_GetActorLocation` (`GameplayStatics.GetPlayerCharacter` 0)))) (`KismetMathLibrary.MakeRotator` 0.0 0.0 (.z `_ローテーション`)) true false))))

(fn `UserConstructionScript`)