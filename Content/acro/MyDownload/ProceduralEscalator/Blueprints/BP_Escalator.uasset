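; Procedural escalator actor that sizes itself from a height setting and runs moving treads up or down.
; Construction places working points, spawns evenly spaced tread mesh components (chosen over instancing for collision) and stretches a spline mesh mid-section.
; While operational, Tick slides treads horizontally, deriving Z from a clamped 30-degree slope.
; End overlap triggers teleport treads back to the opposite toe; CheckForTreadReset's result is unused.
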(event `self.ReceiveTick`
  (params (DeltaSeconds :type "Float (single-precision)"))
  ;[1 1 1] this is where tread movement is handled
  (`self.MoveTreads`))

(event `self.UpperReset.OnComponentBeginOverlap`
  (params (OverlappedComponent :type "PrimitiveComponent Object Reference") (OtherActor :type "Actor Object Reference") (OtherComp :type "PrimitiveComponent Object Reference") (OtherBodyIndex :type Integer) (bFromSweep :type Boolean) (SweepResult :type "HitResult Structure (by ref)"))
  (if (`self.bIsUpEscalator`)
    (if (== OtherActor self)
      (`SceneComponent.K2_SetWorldLocation` OtherComp (`SceneComponent.K2_GetComponentLocation` (`self.LowerToePivot`)) false true))))

(event `self.LowerReset.OnComponentBeginOverlap`
  (params (OverlappedComponent :type "PrimitiveComponent Object Reference") (OtherActor :type "Actor Object Reference") (OtherComp :type "PrimitiveComponent Object Reference") (OtherBodyIndex :type Integer) (bFromSweep :type Boolean) (SweepResult :type "HitResult Structure (by ref)"))
  (if (not (`self.bIsUpEscalator`))
    (if (== OtherActor self)
      (`SceneComponent.K2_SetWorldLocation` OtherComp (`SceneComponent.K2_GetComponentLocation` (`self.UpperToePivot`)) false true))))

(fn `BuildMidSection`
  (bind _returnvalue (`KismetMathLibrary.GetForwardVector` (`self.K2_GetActorRotation`)))
  ;[1 1 1] the mid-section is a spline component, the tangents of which are oriented toward the forward vector of the actor
  (bind _returnvalue_2 (`AddComponent|NODE_AddSplineMeshComponent-1` :`bManualAttachment` true))
  (`SplineMeshComponent.SetStartAndEnd` _returnvalue_2 (`SceneComponent.K2_GetComponentLocation` (`self.TopMesh`)) _returnvalue (`SceneComponent.K2_GetComponentLocation` (`self.BaseMesh`)) _returnvalue true))

(fn `BuildTreadLine`
  (locals (myCurrentTread :type "StaticMeshComponent Object Reference") (myIndex :type Integer))
  (bind _returnvalue (+ (`KismetMathLibrary.SelectVector` (`SceneComponent.K2_GetComponentLocation` (`self.LowerToePivot`)) (`SceneComponent.K2_GetComponentLocation` (`self.UpperToePivot`)) (`self.bIsUpEscalator`)) (* (`SceneComponent.GetForwardVector` (`self.ForwardVector`)) (* (`local.myIndex`) (`self.TreadSpacing`)))))
  ;[1 1 1] Build the tread line based on the total number required determined by the height variable
  (`KismetArrayLibrary.Array_Clear` (`self.TreadList`))
  (for _index (range (+ (`self.TreadCount`) 1))
    (set `local.myIndex` _index)
    (bind _returnvalue_2 (`AddComponent|NODE_AddStaticMeshComponent-1` :`bManualAttachment` true :`RelativeTransform` (`KismetMathLibrary.MakeTransform` (`KismetMathLibrary.MakeVector` (.x _returnvalue) (.y _returnvalue) (`self.CalcZValue` _returnvalue (`local.myIndex`))) (`self.K2_GetActorRotation`)))) ; using a static mesh component instead of an instanced mesh because of better collision mechanics, but slightly higher overhead
    (`KismetArrayLibrary.Array_Add` (`self.TreadList`) _returnvalue_2)))

(fn `CalculateWorkingPoints`
  (bind _height (`self.Height`))
  (bind (_returnvalue_x _returnvalue_y _returnvalue_z) (`KismetMathLibrary.BreakVector` (`SceneComponent.K2_GetComponentLocation` (`self.UpperWorkingPointPivot`))))
  (bind (_relativelocation_x _relativelocation_y _relativelocation_z) (`KismetMathLibrary.BreakVector` (`SceneComponent.RelativeLocation` (`self.LowerWorkingPointPivot`))))
  (bind (_relativelocation_x_2 _relativelocation_y_2 _relativelocation_z_2) (`KismetMathLibrary.BreakVector` (`SceneComponent.RelativeLocation` (`self.UpperWorkingPointPivot`))))
  (`|ExecutionSequence`
    (:`then_0`
      ;[1 1 1] In some cases, the 'forward' direction of the blueprint needs to be determined by the direction of operation
      (`SceneComponent.K2_SetRelativeRotation` (`self.ForwardVector`) (`KismetMathLibrary.SelectRotator` (struct :`Yaw` 180.0) (struct) (`self.bIsUpEscalator`)) false false))
    (:`then_1`
      ;[1 1 1] The top mesh is placed in relation to the requested height.
      (`SceneComponent.K2_SetRelativeLocation` (`self.TopMesh`) (`KismetMathLibrary.MakeVector` (* (`self.EscalatorAngle`) _height -1.0) 0.0 _height) false false))
    (:`then_2`
      ;[1 1 1] The lower toe location is adjusted based on the position of the lower working point
      (`SceneComponent.K2_SetRelativeLocation` (`self.LowerToePivot`) (`KismetMathLibrary.MakeVector` 200.0 _relativelocation_y _relativelocation_z) false false) ; per adjust lower toe
      (`SceneComponent.K2_SetRelativeLocation` (`self.UpperToePivot`) (`KismetMathLibrary.MakeVector` -200.0 _relativelocation_y_2 _relativelocation_z_2) false false) ; pre adjust upper toe
    )
    (:`then_3`
      ;[1 1 1] Estimate the number of treads we need based on escalator run
      (set `self.TreadCount` (`.ReturnValue` (`KismetMathLibrary.FMod` (`self.GetHorizontalDistanceBetweenComps` (`self.LowerToePivot`) (`self.UpperToePivot`)) (`self.TreadSpacing`)))))
    (:`then_4`
      ;[1 1 1] this places the upper toe at an evenly spaced point in front of the upper working point based on the total number treads required
      (`SceneComponent.K2_SetWorldLocation` (`self.UpperToePivot`) (`KismetMathLibrary.MakeVector` (+ (.x (* (* (`KismetMathLibrary.GetForwardVector` (`self.K2_GetActorRotation`)) -1) (* (`self.TreadCount`) (`self.TreadSpacing`)))) (.x (`SceneComponent.K2_GetComponentLocation` (`self.LowerToePivot`)))) (+ (.y (* (* (`KismetMathLibrary.GetForwardVector` (`self.K2_GetActorRotation`)) -1) (* (`self.TreadCount`) (`self.TreadSpacing`)))) (.y (`SceneComponent.K2_GetComponentLocation` (`self.LowerToePivot`)))) _returnvalue_z) false false) ; fine tune upper toe
    )))

(fn `CalcZValue`
  (params (InVector :type "Vector Structure") (TreadIndex :type Integer))
  (returns (ZValue :type "Float (double-precision)"))
  (bind _lowerworkingpointpivot (`self.LowerWorkingPointPivot`))
  (bind (_returnvalue_x _returnvalue_y _returnvalue_z) (`KismetMathLibrary.BreakVector` (`SceneComponent.K2_GetComponentLocation` (`self.LowerWorkingPointPivot`))))
  (bind (_returnvalue_x_2 _returnvalue_y_2 _returnvalue_z_2) (`KismetMathLibrary.BreakVector` (`SceneComponent.K2_GetComponentLocation` (`self.UpperWorkingPointPivot`))))
  (bind (_returnvalue_x_3 _returnvalue_y_3 _returnvalue_z_3) (`KismetMathLibrary.BreakVector` (`SceneComponent.K2_GetComponentLocation` _lowerworkingpointpivot)))
  (bind (_returnvalue_x_4 _returnvalue_y_4) (`KismetMathLibrary.BreakVector` (`SceneComponent.K2_GetComponentLocation` (`self.LowerToePivot`))))
  (return (`KismetMathLibrary.FClamp` (+ (* (`KismetMathLibrary.VSize` (- (`KismetMathLibrary.MakeVector` (.x InVector) (.y InVector)) (`KismetMathLibrary.MakeVector` _returnvalue_x_4 _returnvalue_y_4))) (`KismetMathLibrary.DegTan` 30.0)) (- _returnvalue_z_3 (* (`self.GetHorizontalDistanceBetweenComps` _lowerworkingpointpivot (`self.LowerToePivot`)) (`KismetMathLibrary.DegTan` 30.0)))) _returnvalue_z _returnvalue_z_2)))

(fn `CheckForTreadReset`
  (params (InTreadLoc :type "Vector Structure") (TreadIndex :type Integer))
  (returns (OutVector :type "Vector Structure"))
  (bind _returnvalue (+ TreadIndex -1))
  (bind (_returnvalue_x _returnvalue_y _returnvalue_z) (`KismetMathLibrary.BreakVector` (`SceneComponent.K2_GetComponentLocation` (`self.LowerToePivot`))))
  (bind (_returnvalue_x_2 _returnvalue_y_2 _returnvalue_z_2) (`KismetMathLibrary.BreakVector` (`SceneComponent.K2_GetComponentLocation` (`self.UpperToePivot`))))
  (if (`self.bIsUpEscalator`)
    ;[1 1 1] If moving in the 'up' direction, then see if we're in front of the upper toe.  If we're not, use whatever vector was passed into this function
    (if (`self.IsInFrontOf` InTreadLoc (`SceneComponent.K2_GetComponentLocation` (`self.UpperToePivot`)) (`SceneComponent.GetForwardVector` (`self.ForwardVector`)))
      ;[1 1 1] since we're in front of our forward limit, and need to be reset, we place ourselves directly behind the tread who's index is in front of us
      (return (`KismetMathLibrary.MakeVector` _returnvalue_x _returnvalue_y _returnvalue_z))
      (else
        (return InTreadLoc)))
    (else
      ;[1 1 1] if we're moving in the down direction, see if we're in front of the lower toe.  in this case, the forward vector, is the direction of movement
      (if (`self.IsInFrontOf` InTreadLoc (`SceneComponent.K2_GetComponentLocation` (`self.LowerToePivot`)) (`SceneComponent.GetForwardVector` (`self.ForwardVector`)))
        ;[1 1 1] since we're moving in the down direction, and we need to be reset, we place ourselves in the location directly behind the tread that was indexed behind us
        (return (`KismetMathLibrary.MakeVector` (.x (+ (.location (`SceneComponent.K2_GetComponentToWorld` (`|GetArrayItem` (`self.TreadList`) (`KismetMathLibrary.SelectInt` (- (`self.TreadCount`) 1) _returnvalue (< _returnvalue 0))))) (* (* (`SceneComponent.GetForwardVector` (`self.ForwardVector`)) -1) (`self.TreadSpacing`)))) (.y (+ (.location (`SceneComponent.K2_GetComponentToWorld` (`|GetArrayItem` (`self.TreadList`) (`KismetMathLibrary.SelectInt` (- (`self.TreadCount`) 1) _returnvalue (< _returnvalue 0))))) (* (* (`SceneComponent.GetForwardVector` (`self.ForwardVector`)) -1) (`self.TreadSpacing`)))) _returnvalue_z_2))
        (else
          (return InTreadLoc))))))

(fn `GetHorizontalDistanceBetweenComps`
  (params (CompA :type "SceneComponent Object Reference") (CompB :type "SceneComponent Object Reference"))
  (returns (Distance :type "Float (double-precision)"))
  (return (`KismetMathLibrary.VSize` (- (`KismetMathLibrary.MakeVector` (.x (`SceneComponent.K2_GetComponentLocation` CompA)) (.y (`SceneComponent.K2_GetComponentLocation` CompA))) (`KismetMathLibrary.MakeVector` (.x (`SceneComponent.K2_GetComponentLocation` CompB)) (.y (`SceneComponent.K2_GetComponentLocation` CompB)))))))

(fn `IsInFrontOf`
  (params (VectorA :type "Vector Structure") (VectorB :type "Vector Structure") (ForwardVector :type "Vector Structure"))
  (returns (`bIsInFront?` :type Boolean))
  (return (== (`KismetMathLibrary.Normal` (- (`KismetMathLibrary.MakeVector` (.x VectorA) (.y VectorA)) (`KismetMathLibrary.MakeVector` (.x VectorB) (.y VectorB)))) ForwardVector)))

(fn `MoveTread`
  (params (TreadIndex :type Integer))
  (locals (myNewDistance :type "Float (double-precision)") (myCurrentDistance :type "Float (double-precision)"))
  (bind _escalatorspeed (`self.EscalatorSpeed`))
  (bind _returnvalue (+ (`SceneComponent.K2_GetComponentLocation` (`|GetArrayItem` (`self.TreadList`) TreadIndex)) (* (* (`KismetMathLibrary.GetForwardVector` (`self.K2_GetActorRotation`)) -1) (* (`KismetMathLibrary.SelectFloat` _escalatorspeed (* _escalatorspeed -1.0) (`self.bIsUpEscalator`)) (`GameplayStatics.GetWorldDeltaSeconds`)))))
  ;[1 1 1] Here we calculate the direction of movement, and establish if the tread should be reset based on horizontal position.  The horizontal position also determines where the tread should be located on the Z axis
  (`SceneComponent.K2_SetWorldLocation` (`|GetArrayItem` (`self.TreadList`) TreadIndex) (`KismetMathLibrary.MakeVector` (.x _returnvalue) (.y _returnvalue) (`self.CalcZValue` _returnvalue TreadIndex)) false true))

(fn `MoveTreads`
  (locals (myCurrentTread :type "StaticMeshComponent Object Reference") (myCurrentTreadLoc :type "Float (double-precision)") (myDesiredTreadLoc :type "Float (double-precision)"))
  (if (`self.bOperational`)
    ;[1 1 1] we iterate through each tread and calculate it's next location.  because an iterator is called in tick, this asset can become expensive to use for extremely long escalators
    (for _index (range (`self.TreadCount`))
      (`self.MoveTread` _index))))

(fn `UserConstructionScript`
  (`self.CalculateWorkingPoints`)
  (`self.BuildTreadLine`)
  (`self.BuildMidSection`))