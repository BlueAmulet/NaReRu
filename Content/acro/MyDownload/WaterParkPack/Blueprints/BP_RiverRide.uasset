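; BP_RiverRide is a spline-driven river ride piece for a water park, built entirely in the construction script with no runtime logic.
; It adds a spline mesh between each pair of consecutive spline points, using their locations and tangents for the segment's shape.
; Each segment's up direction is the spline direction rotated -90 degrees around Y, and the final segment swaps to EndMesh.
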(fn `UserConstructionScript`
  (bind _spline (`self.Spline`))
  (bind _returnvalue (- (`SplineComponent.GetNumberOfSplinePoints` _spline) 2))
  (for _index (range (+ _returnvalue 1))
    (bind _returnvalue_2 (`AddComponent|NODE_AddSplineMeshComponent-0`))
    (`SplineMeshComponent.SetSplineUpDir` _returnvalue_2 (`KismetMathLibrary.RotateAngleAxis` (`SplineComponent.GetDirectionAtSplinePoint` _spline _index "Local") -90.0 (0.0 1.0 0.0)) true)
    (`SceneComponent.K2_AttachToComponent` _returnvalue_2 (`self.Scene`) "None" "KeepRelative" "KeepRelative" "KeepRelative" true)
    (bind (_location _tangent) (`SplineComponent.GetLocationAndTangentAtSplinePoint` _spline _index "Local"))
    (bind (_location_2 _tangent_2) (`SplineComponent.GetLocationAndTangentAtSplinePoint` _spline (+ _index 1) "Local"))
    (`SplineMeshComponent.SetStartAndEnd` _returnvalue_2 _location _tangent _location_2 _tangent_2 true)
    (if (== _returnvalue _index)
      (`StaticMeshComponent.SetStaticMesh` _returnvalue_2 (`self.EndMesh`)))))