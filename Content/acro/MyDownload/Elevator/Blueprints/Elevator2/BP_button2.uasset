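; BP_button2 is an elevator floor button that requests a floor from its parent BP_Elevator_Box2 actor.
; PressButton casts the parent actor to the elevator box, adds FloorNumber to its floor queue, then calls TurnOn.
; TurnOn and TurnOff swap the button mesh between lit and unlit materials.
; The construction script applies the configurable StaticMeshButton mesh to the button.
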(event `PressButton`
  ;[1 1 1] Press Button  --> Add floor number to the queue
  (bind _asbp_elevator_box_2 (cast `/Game/acro/MyDownload/Elevator/Blueprints/Elevator2/BP_Elevator_Box2` (`self.GetParentActor`)))
  (`/Game/acro/MyDownload/Elevator/Blueprints/Elevator2/BP_Elevator_Box2.AddToFloorQueue` _asbp_elevator_box_2 (`self.floorNumber`))
  (`self.TurnOn`))

(event `TurnOn`
  ;[1 1 1] Turn On --> Change Material to LIT version
  (`PrimitiveComponent.SetMaterial` (`self.sm_buttons_floor_button-1`) 0 (`self.materialOn`)))

(event `TurnOff`
  ;[1 1 1] Turn Off --> Change Material to UNLIT
  (`PrimitiveComponent.SetMaterial` (`self.sm_buttons_floor_button-1`) 0 (`self.materialOff`)))

(fn `UserConstructionScript`
  (`StaticMeshComponent.SetStaticMesh` (`self.sm_buttons_floor_button-1`) (`self.staticMeshButton`)))