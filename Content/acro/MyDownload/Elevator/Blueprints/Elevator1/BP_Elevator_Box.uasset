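; BP_Elevator_Box is the elevator car, a child actor of BP_Elevator_System that carries players between floors.
; Tick works through a floor queue, moving the car with MoveComponentTo, syncing LED floor displays and playing movement sound.
; On arrival it opens car and floor doors, then closes them on a timer, reopening on player overlap or blocking hits.
; It also prunes surplus floor buttons and toggles the escape hatch and glass material.
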(event `closeHatch`
  (bind _sm_escapehatch (`self.sm_escapeHatch`))
  ;[1 1 1] エスケープハッチを閉じる/開く
  (`KismetSystemLibrary.MoveComponentTo` _sm_escapehatch (`SceneComponent.RelativeLocation` _sm_escapehatch))
  (`SceneComponent.SetVisibility` (`self.sm_hatchCover`) true false))

(event `openHatch`
  (bind _sm_escapehatch (`self.sm_escapeHatch`))
  ;[1 1 1] エスケープハッチを閉じる/開く
  (`KismetSystemLibrary.MoveComponentTo` _sm_escapehatch (`SceneComponent.RelativeLocation` _sm_escapehatch) (struct :`Roll` -90.0) :!label _label)
  (`SceneComponent.SetVisibility` (`self.sm_hatchCover`) false false))

(event `カスタムイベント_0`
  ;[1 1 1] エスケープハッチを閉じる/開く
  (goto _label))

(event `self.ReceiveBeginPlay`
  (bind _returnvalue (`self.K2_GetComponentsByClass` (`GameplayStatics.GetObjectClass` (`self.BP_button01`))))
  ;[1 1 1] Initialize variables
  (bind _asbp_elevator_system (cast `/Game/acro/MyDownload/Elevator/Blueprints/Elevator1/BP_Elevator_System` (`self.GetParentActor`)))
  (`|ExecutionSequence`
    (:`then_0`
      (set `self.timeToWaitAtFloor` (`/Game/acro/MyDownload/Elevator/Blueprints/Elevator1/BP_Elevator_System.timeToWaitAtFloors` _asbp_elevator_system)))
    (:`then_1`
      (set `self.waitAtFloorUntil` 0.0)
      (set `self.rightDoorClosedPosition` (`SceneComponent.RelativeLocation` (`self.rightDoor`)))
      (set `self.leftDoorClosedPosition` (`SceneComponent.RelativeLocation` (`self.leftDoor`)))
      (set `self.rightDoorOpen_WorldPosition` (`SceneComponent.K2_GetComponentLocation` (`self.rightDoor`)))
      (set `self.leftDoorOpen_WorldPosition` (`SceneComponent.K2_GetComponentLocation` (`self.leftDoor`)))
      ;;[1 1 1] エレベータ内の余分なボタンを取り除いてください。エレベーターシステムの実際の階数に対応したボタンの数だけ残しています
      (for _array_element _returnvalue
        (bind _asbp_button (cast `/Game/acro/MyDownload/Elevator/Blueprints/Elevator1/BP_button` (`ChildActorComponent.ChildActor` _array_element)))
        (bind _asbp_elevator_system_2 (cast `/Game/acro/MyDownload/Elevator/Blueprints/Elevator1/BP_Elevator_System` (`self.GetParentActor`)))
        (if (> (`/Game/acro/MyDownload/Elevator/Blueprints/Elevator1/BP_button.floorNumber` _asbp_button) (- (`KismetArrayLibrary.Array_Length` (`/Game/acro/MyDownload/Elevator/Blueprints/Elevator1/BP_Elevator_System.arrayDoorFrames` _asbp_elevator_system_2)) 1))
          (`self.K2_DestroyActor` _asbp_button)
          ;[1 1 1] インスタンスごとにボタンの位置を良くするために、ボタンにオフセットを適用します。
          (for _array_element_2 _returnvalue
            (`SceneComponent.K2_AddRelativeLocation` _array_element_2 (`/Game/acro/MyDownload/Elevator/Blueprints/Elevator1/BP_Elevator_System.buttonOffsetPosition` _asbp_elevator_system) false true)))))
    (:`then_2`
      (set `self.doorSpeed` (/ 2.0 (`/Game/acro/MyDownload/Elevator/Blueprints/Elevator1/BP_Elevator_System.doorSpeed` _asbp_elevator_system))))
    (:`then_3`
      (set `self.elevatorSpeed` (/ 2.0 (`/Game/acro/MyDownload/Elevator/Blueprints/Elevator1/BP_Elevator_System.elevatorSpeed` _asbp_elevator_system))))))

(event `通常化`
  ;[1 1 1] エレベーター透過
  (`PrimitiveComponent.SetMaterial` (`self.ElevatorMesh`) 0 "/Game/acro/MyDownload/Elevator/Materials/1/M_ElevatorBox_1.M_ElevatorBox_1"))

(event `透明化`
  ;[1 1 1] エレベーター透過
  (`PrimitiveComponent.SetMaterial` (`self.ElevatorMesh`) 0 "/Game/shinkansen/Kento/shinkansen/Airbus_Glass.Airbus_Glass"))

(event `SetFloorLEDDisplay`
  (params (currentFloor :type Integer))
  (bind _returnvalue (- currentFloor 1))
  (bind _material_leddisplay (`self.Material_LEDDisplay`))
  ;[1 1 1] 現在の階数を表示するようにLED表示を設定します。
  (`MaterialInstanceDynamic.SetScalarParameterValue` _material_leddisplay "TextureOffset_U" (* (`KismetMathLibrary.Conv_IntToDouble` (`.ReturnValue` (`KismetMathLibrary.FMod` (`KismetMathLibrary.Conv_IntToDouble` _returnvalue) 10.0))) 0.1))
  (`MaterialInstanceDynamic.SetScalarParameterValue` _material_leddisplay "TextureOffset_V" (* (mod _returnvalue 10) 0.1)))

(event `eventCloseDoors`
  ;[1 1 1] ドアを閉める
  (if (>= (`KismetArrayLibrary.Array_Length` (`PrimitiveComponent.GetOverlappingActors` (`self.PlayerTrigger`) null)) 1)
    (`self.eventOpenDoors`)
    (else
      (set `self.doorsClosing` true)
      (set `self.closeDoorTime` (+ (`KismetSystemLibrary.GetGameTimeInSeconds`) 10000000000.0))
      (`|ExecutionSequence`
        (:`then_0`
          (`KismetSystemLibrary.MoveComponentTo` (`self.rightDoor`) (`self.rightDoorClosedPosition`) (struct) false false (`self.doorSpeed`)))
        (:`then_1`
          (`KismetSystemLibrary.MoveComponentTo` (`self.leftDoor`) (`self.leftDoorClosedPosition`) (struct) false false (`self.doorSpeed`))))
      (set `self.doorsClosing` false))))

(event `eventOpenDoors`
  (bind _rightdoor (`self.rightDoor`))
  (bind _leftdoor (`self.leftDoor`))
  ;[1 1 1] ドアを開ける
  (set `self.doorsOpening` true)
  (set `self.waitAtFloorUntil` (+ (`KismetSystemLibrary.GetGameTimeInSeconds`) (`self.timeToWaitAtFloor`) (`self.doorSpeed`)))
  (set `self.closeDoorTime` (+ (`KismetSystemLibrary.GetGameTimeInSeconds`) (`self.timeToWaitAtFloor`)))
  (`|ExecutionSequence`
    (:`then_0`
      (set `self.rightDoorOpen_WorldPosition` (`SceneComponent.K2_GetComponentLocation` _rightdoor))
      (`KismetSystemLibrary.MoveComponentTo` _rightdoor (`self.rightDoorOpenPosition`) (struct) false false (`self.doorSpeed`))
      (set `self.doorsOpening` false))
    (:`then_1`
      (set `self.leftDoorOpen_WorldPosition` (`SceneComponent.K2_GetComponentLocation` _leftdoor))
      (`KismetSystemLibrary.MoveComponentTo` _leftdoor (`self.leftDoorOpenPosition`) (struct) false false (`self.doorSpeed`)))))

(event `eventMoveToFloor`
  (params (height :type "Float (double-precision)"))
  ;[1 1 1] エレベーターを目的の階に移動させる
  (`KismetSystemLibrary.MoveComponentTo` (`self.ElevatorMesh`) (`KismetMathLibrary.MakeVector` 0.0 0.0 height) (struct) false false (* (/ (`KismetMathLibrary.Abs` (- (.z (`SceneComponent.RelativeLocation` (`self.ElevatorMesh`))) height)) 300.0) (`self.elevatorSpeed`)))
  (bind _foundwidgets (`WidgetBlueprintLibrary.GetAllWidgetsOfClass` "/Game/acro/VR_Spectator_Window/AcroWindow.AcroWindow_C" false))
  (`/Game/acro/VR_Spectator_Window/AcroWindow.kaisou_Button_on` _foundwidgets))

(event `self.ReceiveTick`
  (params (DeltaSeconds :type "Float (single-precision)"))
  (bind _move_loop_cue (`self.move_loop_Cue`))
  (bind _returnvalue (`SceneComponent.K2_GetComponentLocation` (`self.ElevatorMesh`)))
  (bind _returnvalue_2 (`AudioComponent.IsPlaying` _move_loop_cue))
  ;[1 1 1] EVENT TICK
  (`|ExecutionSequence`
    (:`then_0`
      ;[1 1 1] フロアに到着したかどうかの確認
      (if (and (not (`self.waitingAtFloor`)) (<= (`KismetMathLibrary.Abs` (- (`self.currentFloorTargetHeight`) (.z (`SceneComponent.RelativeLocation` (`self.ElevatorMesh`))))) 5.0) (> (`KismetArrayLibrary.Array_Length` (`self.floorQueue`)) 0))
        (`self.ArrivedAtFloor`)
        (else
          ;[1 1 1] 到着した階数を決める
          (for (_array_element _array_index) (`self.arrayFloors`)
            ;[1 1 1] 現在の階数を表示するようにLEDを設定します。
            (if (and (<= (`KismetMathLibrary.Abs` (- (.z (`SceneComponent.RelativeLocation` (`self.ElevatorMesh`))) _array_element)) 100.0) (> _array_index 0))
              (if (!= (`self.currentFloorNumber`) _array_index)
                (bind _output_get (set `self.currentFloorNumber` _array_index))
                (bind _asbp_elevator_system (cast `/Game/acro/MyDownload/Elevator/Blueprints/Elevator1/BP_Elevator_System` (`self.GetParentActor`)))
                (`/Game/acro/MyDownload/Elevator/Blueprints/Elevator1/BP_Elevator_System.SetAllDoorFrames_LEDDisplay` _asbp_elevator_system _output_get)
                (`self.SetFloorLEDDisplay` _output_get)))))))
    (:`then_1`
      ;[1 1 1] フロアのキューが空いていないか、待ち時間が過ぎていないか確認してください。
      (if (and (> (`KismetArrayLibrary.Array_Length` (`self.floorQueue`)) 0) (<= (`self.waitAtFloorUntil`) (`KismetSystemLibrary.GetGameTimeInSeconds`)))
        (`self.MoveToFloor`)))
    (:`then_2`
      ;[1 1 1] 待ち時間が過ぎたらドアを閉める
      (if (<= (`self.closeDoorTime`) (`KismetSystemLibrary.GetGameTimeInSeconds`))
        (`self.eventCloseDoors`)))
    (:`then_3`
      ;[1 1 1] エレベーターの移動音を再生する
      (bind _output_get_2 (set `self.currentSpeed` (`KismetMathLibrary.VSize` (- _returnvalue (`self.lastElevatorPos`)))))
      (set `self.lastElevatorPos` _returnvalue)
      (if (>= _output_get_2 0.5)
        (if (not _returnvalue_2)
          (`AudioComponent.Play` _move_loop_cue 0.0))
        (elif _returnvalue_2
          (`AudioComponent.Stop` _move_loop_cue))))))

(event `self.leftDoor.OnComponentHit`
  (params (HitComponent :type "PrimitiveComponent Object Reference") (OtherActor :type "Actor Object Reference") (OtherComp :type "PrimitiveComponent Object Reference") (NormalImpulse :type "Vector Structure") (Hit :type "HitResult Structure (by ref)"))
  (bind _returnvalue (`SceneComponent.K2_GetComponentLocation` (`self.leftDoor`)))
  (bind _returnvalue_2 (`SceneComponent.K2_GetComponentLocation` (`self.rightDoor`)))
  ;[1 1 1] ドアが閉まらないように物理オブジェクトがあるかどうか確認してください
  (if (and (`self.doorsClosing`) (or (<= (`KismetMathLibrary.Dot_VectorVector` (`KismetMathLibrary.Normal` (- (`.ImpactPoint` (`GameplayStatics.BreakHitResult` Hit)) _returnvalue)) (`KismetMathLibrary.Normal` (- _returnvalue (`self.leftDoorOpen_WorldPosition`)))) -0.75) (<= (`KismetMathLibrary.Dot_VectorVector` (`KismetMathLibrary.Normal` (- (`.ImpactPoint` (`GameplayStatics.BreakHitResult` (stale `self.rightDoor.OnComponentHit` Hit))) _returnvalue_2)) (`KismetMathLibrary.Normal` (- _returnvalue_2 (`self.rightDoorOpen_WorldPosition`)))) -0.75)) (not (`self.doorsOpening`))) :!label _label_2
    (`self.eventOpenDoors`)))

(event `self.rightDoor.OnComponentHit`
  (params (HitComponent :type "PrimitiveComponent Object Reference") (OtherActor :type "Actor Object Reference") (OtherComp :type "PrimitiveComponent Object Reference") (NormalImpulse :type "Vector Structure") (Hit :type "HitResult Structure (by ref)"))
  ;[1 1 1] ドアが閉まらないように物理オブジェクトがあるかどうか確認してください
  (goto _label_2))

(fn `AddToFloorQueue`
  (params (floorToAdd :type Integer))
  ;[1 1 1] If the floor is not already in the queue of floors we're visiting, Add it to the QUEUE
  (if (not (`KismetArrayLibrary.Array_Contains` (`self.floorQueue`) floorToAdd))
    (`KismetArrayLibrary.Array_Add` (`self.floorQueue`) floorToAdd)))

(fn `ArrivedAtFloor`
  (`GameplayStatics.SpawnSoundAttached` "/Game/acro/MyDownload/Elevator/Sounds/floor_ring.floor_ring" (`self.Audio`) "None" (0.0 0.0 0.0) (struct) "KeepRelativeOffset" false 1.0 1.0 0.0 null null)
  (set `self.waitingAtFloor` true)
  ;[1 1 1] Open the doors of the floor we just arrived at
  (bind _asbp_elevator_system (cast `/Game/acro/MyDownload/Elevator/Blueprints/Elevator1/BP_Elevator_System` (`self.GetParentActor`)))
  (`/Game/acro/MyDownload/Elevator/Blueprints/Elevator1/BP_DoorFrame.eventOpenDoors` (`|GetArrayItem` (`/Game/acro/MyDownload/Elevator/Blueprints/Elevator1/BP_Elevator_System.arrayDoorFrames` _asbp_elevator_system) (`self.currentFloorTarget`)))
  ;[1 1 1] Remove the floor we just arrived at from the QUEUE
  (`KismetArrayLibrary.Array_RemoveItem` (`self.floorQueue`) (`self.currentFloorTarget`))
  (`self.eventOpenDoors`)
  ;[1 1 1] Find the floor button for the floor we just arrived at and turn it off
  (for _array_element (`self.K2_GetComponentsByClass` (`GameplayStatics.GetObjectClass` (`self.BP_button01`)))
    (bind _asbp_button (cast `/Game/acro/MyDownload/Elevator/Blueprints/Elevator1/BP_button` (`ChildActorComponent.ChildActor` _array_element)))
    (`/Engine/EditorBlueprintResources/StandardMacros.IsValid` _asbp_button
      (:`Is Valid`
        (if (== (`/Game/acro/MyDownload/Elevator/Blueprints/Elevator1/BP_button.floorNumber` _asbp_button) (`self.currentFloorTarget`))
          (`/Game/acro/MyDownload/Elevator/Blueprints/Elevator1/BP_button.TurnOff` _asbp_button))))))

(fn `MoveToFloor`
  ;[1 1 1] Grab the next floor to head towards
  (bind _output_get (set `self.currentFloorTarget` (`|GetArrayItem` (`self.floorQueue`))))
  (set `self.waitingAtFloor` false)
  (bind _output_get_2 (set `self.currentFloorTargetHeight` (`|GetArrayItem` (`self.arrayFloors`) _output_get)))
  (`self.eventMoveToFloor` _output_get_2))

(fn `UserConstructionScript`
  (bind _returnvalue (`PrimitiveComponent.CreateDynamicMaterialInstance` (`self.ElevatorMesh`) 1 null "None"))
  (set `self.Material_LEDDisplay` _returnvalue))