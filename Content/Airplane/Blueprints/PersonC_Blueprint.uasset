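; PersonC is a character Blueprint in the Airplane folder that randomly varies its sitting animation.
; From BeginPlay it loops indefinitely, waiting a random 5 to 15 seconds before each run of the アニメーション割合制御_2_2 macro.
; The macro picks one of three equally likely values and writes it to SitAnimValue on the skeletal mesh's SubwaySit_AnimBP instance.
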(event `self.ReceiveBeginPlay`
  (bind _returnvalue (`SkeletalMeshComponent.GetAnimInstance` (`self.SkeletalMeshComponent`)))
  ;[1 1 1] アニメーション変更
  (`KismetSystemLibrary.Delay` (`KismetMathLibrary.RandomFloatInRange` 5.0 15.0) :!label _label)
  (switch `int` (`KismetMathLibrary.RandomInteger` 3)
    (:`0`
      (bind _assubway_sit_anim_bp (cast `/Game/Subway/Animation/SubwaySit_AnimBP` _returnvalue))
      (set `/Game/Subway/Animation/SubwaySit_AnimBP.SitAnimValue` 0 _assubway_sit_anim_bp)
      (goto _label))
    (:`1`
      (bind _assubway_sit_anim_bp_2 (cast `/Game/Subway/Animation/SubwaySit_AnimBP` _returnvalue))
      (set `/Game/Subway/Animation/SubwaySit_AnimBP.SitAnimValue` 1 _assubway_sit_anim_bp_2)
      (goto _label))
    (:`2`
      (bind _assubway_sit_anim_bp_3 (cast `/Game/Subway/Animation/SubwaySit_AnimBP` _returnvalue))
      (set `/Game/Subway/Animation/SubwaySit_AnimBP.SitAnimValue` 2 _assubway_sit_anim_bp_3)
      (goto _label))))

(fn `UserConstructionScript`)