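; Interviewer character Blueprint for a job interview, where keyboard keys trigger spoken questions, a seating prompt and a closing line.
; Each key sets a Question index that selects a voice clip and starts its lip sync data.
; OnVisemesReady events write five scaled visemes to the same Mouth_Open morph, plus Eye_Blink from a timeline that nothing here starts.
; The seating and closing keys also step SitAnimValue on Interview_AnimBP.
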(event Input|KeyboardEvents|Multiply
  (params (Key :type Key%20Structure))
  (:Pressed
    (bind _asinterview_anim_bp (Utilities|Casting|CastToInterview_AnimBP (Components|SkeletalMesh|GetAnimInstance (Variables|SkeletalMeshActor|GetSkeletalMeshComponent))))
    (Variables|/Game/Interview/Blueprints/Interview_AnimBP.Interview_AnimBP_C|SetSitAnimValue _asinterview_anim_bp 4) ; ありがとうございました
  ))

(event Input|KeyboardEvents|Divide
  (params (Key :type Key%20Structure))
  (:Pressed
    (bind _asinterview_anim_bp (Utilities|Casting|CastToInterview_AnimBP (Components|SkeletalMesh|GetAnimInstance (Variables|SkeletalMeshActor|GetSkeletalMeshComponent))))
    (Variables|/Game/Interview/Blueprints/Interview_AnimBP.Interview_AnimBP_C|SetSitAnimValue _asinterview_anim_bp 1) ; どうぞおかけください
    (Utilities|FlowControl|Delay 1.5)
    (Variables|/Game/Interview/Blueprints/Interview_AnimBP.Interview_AnimBP_C|SetSitAnimValue _asinterview_anim_bp 2) ; 座るモーション
    (Utilities|FlowControl|Delay 0.7)
    (Variables|/Game/Interview/Blueprints/Interview_AnimBP.Interview_AnimBP_C|SetSitAnimValue _asinterview_anim_bp 3) ; 書類を読むモーション
  ))

(fn ConstructionScript)

(event Input|KeyboardEvents|B
  (params (Key :type Key%20Structure))
  (:Pressed
    (Variables|Default|SetQuestion 16)
    (|Outputs) ; enters at 成功/失敗体験を教えてください
  ))

(event Input|KeyboardEvents|N
  (params (Key :type Key%20Structure))
  (:Pressed
    (Variables|Default|SetQuestion 17)
    (|Outputs) ; enters at 挫折した経験はありますか
  ))

(event Input|KeyboardEvents|Enter
  (params (Key :type Key%20Structure))
  (:Pressed
    (Variables|Default|SetQuestion 0)
    (return)))

(event Input|KeyboardEvents|Decimal
  (params (Key :type Key%20Structure))
  (:Pressed
    (Variables|Default|SetQuestion 1)
    (|Outputs) ; enters at 自己PRをお願いします
  ))

(event Input|KeyboardEvents|0
  (params (Key :type Key%20Structure))
  (:Pressed
    (Variables|Default|SetQuestion 2)
    (|Outputs) ; enters at [学生]学生時代頑張ったことは何ですか
  ))

(event Input|KeyboardEvents|1
  (params (Key :type Key%20Structure))
  (:Pressed
    (Variables|Default|SetQuestion 3)
    (|Outputs) ; enters at [社会人]職務経歴を教えてください
  ))

(event Input|KeyboardEvents|2
  (params (Key :type Key%20Structure))
  (:Pressed
    (Variables|Default|SetQuestion 4)
    (|Outputs) ; enters at [社会人]前職の退職理由は何ですか
  ))

(event Input|KeyboardEvents|3
  (params (Key :type Key%20Structure))
  (:Pressed
    (Variables|Default|SetQuestion 5)
    (|Outputs) ; enters at この業界を志望した理由は何ですか
  ))

(event Input|KeyboardEvents|4
  (params (Key :type Key%20Structure))
  (:Pressed
    (Variables|Default|SetQuestion 6)
    (|Outputs) ; enters at 当社を志望した理由は何ですか
  ))

(event Input|KeyboardEvents|5
  (params (Key :type Key%20Structure))
  (:Pressed
    (Variables|Default|SetQuestion 7)
    (|Outputs) ; enters at 趣味は何ですか
  ))

(event Input|KeyboardEvents|6
  (params (Key :type Key%20Structure))
  (:Pressed
    (Variables|Default|SetQuestion 8)
    (|Outputs) ; enters at 今までで一番感動したことはなんですか
  ))

(event Input|KeyboardEvents|7
  (params (Key :type Key%20Structure))
  (:Pressed
    (Variables|Default|SetQuestion 9)
    (|Outputs) ; enters at 今までで一番悔しかったことはなんですか
  ))

(event Input|KeyboardEvents|8
  (params (Key :type Key%20Structure))
  (:Pressed
    (Variables|Default|SetQuestion 10)
    (|Outputs) ; enters at 長所/短所を教えてください
  ))

(event Input|KeyboardEvents|9
  (params (Key :type Key%20Structure))
  (:Pressed
    (Variables|Default|SetQuestion 11)
    (|Outputs) ; enters at キャリアプランはありますか
  ))

(event Input|KeyboardEvents|M
  (params (Key :type Key%20Structure))
  (:Pressed
    (Variables|Default|SetQuestion 18)
    (|Outputs) ; enters at 企業選びの軸は何ですか
  ))

(event Input|KeyboardEvents|Multiply
  (params (Key :type Key%20Structure))
  (:Pressed
    (Variables|Default|SetQuestion 22)
    (|Outputs) ; enters at 面接ありがとうございました
  ))

(event Input|KeyboardEvents|G
  (params (Key :type Key%20Structure))
  (:Pressed
    (Variables|Default|SetQuestion 20)
    (|Outputs) ; enters at 5年後はどうなっていたいですか
  ))

(event Input|KeyboardEvents|Divide
  (params (Key :type Key%20Structure))
  (:Pressed
    (Variables|Default|SetQuestion 21)
    (|Outputs) ; enters at どうぞおかけください
  ))

(event Input|KeyboardEvents|F
  (params (Key :type Key%20Structure))
  (:Pressed
    (Variables|Default|SetQuestion 19)
    (|Outputs) ; enters at 入社後にやりたい仕事は何ですか
  ))

(event Input|KeyboardEvents|Z
  (params (Key :type Key%20Structure))
  (:Pressed
    (Variables|Default|SetQuestion 12)
    (|Outputs) ; enters at 今までの仕事にどんな不満を持っていましたか
  ))

(event Input|KeyboardEvents|X
  (params (Key :type Key%20Structure))
  (:Pressed
    (Variables|Default|SetQuestion 13)
    (|Outputs) ; enters at 当社があなたを採用するメリットは何ですか
  ))

(event Input|KeyboardEvents|C
  (params (Key :type Key%20Structure))
  (:Pressed
    (Variables|Default|SetQuestion 14)
    (|Outputs) ; enters at あなたは周りからどのように評価されていますか
  ))

(event Input|KeyboardEvents|V
  (params (Key :type Key%20Structure))
  (:Pressed
    (Variables|Default|SetQuestion 15)
    (|Outputs) ; enters at リーダーシップを取った経験はありますか
  ))

(event OnVisemesReady(どうぞおかけください[シーケンス])
  (|Outputs) ; enters at どうぞおかけください
)

(event OnVisemesReady(面接ありがとうございました[シーケンス])
  (|Outputs) ; enters at 面接ありがとうございました
)

(event OnVisemesReady(今までの仕事にどんな不満を持っていましたか[シーケンス])
  (|Outputs) ; enters at 今までの仕事にどんな不満を持っていましたか
)

(event OnVisemesReady(当社があなたを採用するメリットは何ですか[シーケンス])
  (|Outputs) ; enters at 当社があなたを採用するメリットは何ですか
)

(event OnVisemesReady(あなたは周りからどのように評価されていますか[シーケンス])
  (|Outputs) ; enters at あなたは周りからどのように評価されていますか
)

(event OnVisemesReady(リーダーシップを取った経験はありますか[シーケンス])
  (|Outputs) ; enters at リーダーシップを取った経験はありますか
)

(event OnVisemesReady(成功/失敗体験を教えてください[シーケンス])
  (|Outputs) ; enters at 成功/失敗体験を教えてください
)

(event OnVisemesReady(挫折した経験はありますか[シーケンス])
  (|Outputs) ; enters at 挫折した経験はありますか
)

(event OnVisemesReady(企業選びの軸は何ですか[シーケンス])
  (|Outputs) ; enters at 企業選びの軸は何ですか
)

(event OnVisemesReady(入社後にやりたい仕事は何ですか[シーケンス])
  (|Outputs) ; enters at 入社後にやりたい仕事は何ですか
)

(event OnVisemesReady(5年後はどうなっていたいですか[シーケンス])
  (|Outputs) ; enters at 5年後はどうなっていたいですか
)

(event OnVisemesReady(自己PRをお願いします[シーケンス])
  (|Outputs) ; enters at 自己PRをお願いします
)

(event OnVisemesReady([社会人]職務経歴を教えてください[シーケンス])
  (|Outputs) ; enters at [社会人]前職の退職理由は何ですか
)

(event OnVisemesReady([学生]学生時代頑張ったことは何ですか[シーケンス])
  (|Outputs) ; enters at [学生]学生時代頑張ったことは何ですか
)

(event OnVisemesReady(自己紹介をお願いします[シーケンス])
  (return))

(event OnVisemesReady(当社を志望した理由は何ですか[シーケンス])
  (|Outputs) ; enters at [社会人]職務経歴を教えてください
)

(event OnVisemesReady([社会人]前職の退職理由は何ですか[シーケンス])
  (|Outputs) ; enters at この業界を志望した理由は何ですか
)

(event OnVisemesReady(この業界を志望した理由は何ですか[シーケンス])
  (|Outputs) ; enters at 当社を志望した理由は何ですか
)

(event OnVisemesReady(趣味は何ですか[シーケンス])
  (|Outputs) ; enters at 趣味は何ですか
)

(event OnVisemesReady(今までで一番感動したことはなんですか[シーケンス])
  (|Outputs) ; enters at 今までで一番感動したことはなんですか
)

(event OnVisemesReady(今までで一番悔しかったことはなんですか[シーケンス])
  (|Outputs) ; enters at 今までで一番悔しかったことはなんですか
)

(event OnVisemesReady(長所/短所を教えてください[シーケンス])
  (|Outputs) ; enters at 長所/短所を教えてください
)

(event OnVisemesReady(キャリアプランはありますか[シーケンス])
  (|Outputs) ; enters at キャリアプランはありますか
)