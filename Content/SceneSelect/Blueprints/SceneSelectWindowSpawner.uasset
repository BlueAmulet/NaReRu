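; Scene-select Blueprint with airplane, subway, Shinkansen and bus events that lead to their travel levels, and a windowed 800x600 resolution set on BeginPlay.
; Each event plays the shared player-move timeline, which moves and turns the player character and sets a Door flag, then opens a level after a delay.
; The subway and Shinkansen events open each other's levels.
; White camera-fade macros exist, but their calls never run.
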(event `self.ReceiveBeginPlay`
  (`KismetSystemLibrary.ExecuteConsoleCommand` "r.SetRes 800x600w" null))

(event `飛行機`
  (`|ExecutionSequence`
    (:`then_0`
      (bind (_direction `_移動`) (`Timeline|プレイヤー移動` :!via `PlayFromStart` :!label _label)
        (:`Update`
          (`self.K2_SetActorLocationAndRotation` (`GameplayStatics.GetPlayerCharacter` 0) (`KismetMathLibrary.MakeVector` (.x `_移動`) (.y `_移動`) (.z (`self.K2_GetActorLocation` (`GameplayStatics.GetPlayerCharacter` 0)))) (struct :`Yaw` 90.0) false false))
        (:`ドア開ける`
          (set `self.Door` true))))
    (:`then_1`
      (`KismetSystemLibrary.Delay` 8.0)
      (`GameplayStatics.OpenLevel` "Plane_Master"))))

(event `地下鉄`
  (`|ExecutionSequence`
    (:`then_0`
      (goto _label :!via `PlayFromStart`))
    (:`then_1`
      (`KismetSystemLibrary.Delay` 8.0)
      (`GameplayStatics.OpenLevel` "Shinkansen_Master"))))

(event `新幹線`
  (`|ExecutionSequence`
    (:`then_0`
      (goto _label :!via `PlayFromStart`))
    (:`then_1`
      (`KismetSystemLibrary.Delay` 8.0)
      (`GameplayStatics.OpenLevel` "Subway_Master"))))

(event `バス`
  (`|ExecutionSequence`
    (:`then_0`
      (goto _label :!via `PlayFromStart`))
    (:`then_1`
      (`KismetSystemLibrary.Delay` 8.0)
      (`GameplayStatics.OpenLevel` "Bus_Master"))))

(fn `UserConstructionScript`)