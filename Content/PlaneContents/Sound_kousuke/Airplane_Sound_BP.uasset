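; Airplane sound Blueprint that plays a beep cue and a crossfade engine recording, exposing events that drive the recording's AISAC controls (CRI ADX2).
; Separate events start playback, fade in high noise, raise its tune after a delay, and switch to flying by raising that control while fading high noise out.
; Delay-based loop macros step each value toward its limit, pushing it to the cue on every tick.
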(event `Play_sound_Airplane_beep`
  ;[1 1 1] Play_and_Init
  (`AtomComponent.Play` (`self.Airplane_beep_cue`) 0.0))

(event `Play_sound_Airplane_rec_crossfade`
  ;[1 1 1] Play_and_Init
  (bind _output_get (set `self.Clossfade` 0.0))
  (`AtomComponent.SetAisacByName` (`self.Airplane_rec_crossfade`) "AisacControl_01" _output_get)
  (`AtomComponent.Play` (`self.Airplane_rec_crossfade`) 0.0))

(event `Set_Aisac_Airplane_highnoise_vol`
  (`self.Loop_HighNoise_Vol_up`
    (:`Loop`
      (bind _output_get (set `self.Clossfade` (+ (`self.Clossfade`) 0.01)))
      (`AtomComponent.SetAisacByName` (`self.Airplane_rec_crossfade`) "AisacControl_01" _output_get))
    (:`End`
      (`KismetSystemLibrary.PrintString` "Set Aisac_HighNoise_Compiled"))))

(event `Set_Aisac_Airplane_highnoise_tune`
  (`KismetSystemLibrary.Delay` 15.0)
  (`self.Loop_HighNoise_Tune`
    (:`Loop`
      (bind _output_get (set `self.Tune` (+ (`self.Tune`) 0.1)))
      (`AtomComponent.SetAisacByName` (`self.Airplane_rec_crossfade`) "AisacControl_02" _output_get))
    (:`End`
      (`KismetSystemLibrary.PrintString` "Set_Aisac_HighNoise_Tune_Compiled"))))

(event `Set_Aisac_Airplane_flying`
  (`|ExecutionSequence`
    (:`then_0`
      (`self.Loop_Flying`
        (:`Loop`
          (bind _output_get (set `self.Flying` (+ (`self.Flying`) 0.01)))
          (`AtomComponent.SetAisacByName` (`self.Airplane_rec_crossfade`) "AisacControl_10" _output_get))
        (:`End`
          (`KismetSystemLibrary.PrintString` "Set_Aisac_Flying_Compiled"))))
    (:`then_1`
      (`self.Loop_HighNoise_Vol_down`
        (:`Loop`
          (bind _output_get_2 (set `self.Clossfade` (- (`self.Clossfade`) 0.01)))
          (`AtomComponent.SetAisacByName` (`self.Airplane_rec_crossfade`) "AisacControl_01" _output_get_2))
        (:`End`
          (`KismetSystemLibrary.PrintString` "Set Aisac_HighNoise_Compiled"))))))

(fn `UserConstructionScript`)