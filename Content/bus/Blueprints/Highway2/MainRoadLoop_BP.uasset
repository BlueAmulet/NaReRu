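; MainRoadLoop_BP is a moving highway segment that forms a self-replenishing road loop.
; On BeginPlay a timeline drives its relative location, and an event track spawns the next copy at a fixed position.
; It destroys itself ten seconds after the timeline finishes, or when Bus_SpectatorWindow's gate-spawn dispatcher fires for the terminal gate.
; Random building-visibility logic is present but unconnected.
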(event `self.ReceiveBeginPlay`
  (bind _outactors (`GameplayStatics.GetAllActorsOfClass` "/Game/bus/VR_Spectator_Window/Bus_SpectatorWindow.Bus_SpectatorWindow_C"))
  (add `/Game/bus/VR_Spectator_Window/Bus_SpectatorWindow.ゲートスポーン` _outactors (delegate `終着ゲート`))
  (bind (_direction _starttimeline) (`Timeline|タイムライン_道` :!via `PlayFromStart`)
    (:`Update`
      (`self.K2_SetActorRelativeLocation` _starttimeline))
    (:`Finished`
      (`KismetSystemLibrary.Delay` 10.0)
      (`self.K2_DestroyActor`))
    (:`道路スポーン`
      (`|SpawnActorFromClass` "MainRoadLoop_BP_C" (`KismetMathLibrary.MakeTransform` (130.0 40430.0 -90.0)) "Undefined" "OverrideRootScale" null null))))

(event `終着ゲート`
  (`self.K2_DestroyActor`))

(fn `UserConstructionScript`)