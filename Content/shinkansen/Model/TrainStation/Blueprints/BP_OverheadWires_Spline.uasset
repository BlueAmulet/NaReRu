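; Train station overhead wire builder that places poles along a spline and strings cables between them.
; The construction script spawns a BP_OverheadWires child actor at each spline point's local location and stores it in an array.
; A second loop snaps each pole's Cable1 and Cable2 to the next pole's Con1 and Con2, chaining the wires along the spline.
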(fn `UserConstructionScript`
  ;[1 1 1] Gets and sets number of spline points
  (bind _output_get (set `self.Number Of Spline Points` (- (`SplineComponent.GetNumberOfSplinePoints` (`self.Spline`)) 0)))
  (for _index (range (+ _output_get 1))
    (set `self.Index of Loop` _index)
    ;[1 1 1] Grabs BP_Overhead_Wires and uses as a child actor.
    (bind _returnvalue (`AddComponent|NODE_AddChildActorComponent-1` :`RelativeTransform` (`KismetMathLibrary.Conv_VectorToTransform` (`SplineComponent.GetLocationAtSplinePoint` (`self.Spline`) (`self.Index of Loop`) "Local"))))
    (`ChildActorComponent.SetChildActorClass` _returnvalue "/Game/Shinkansen/Model/TrainStation/Blueprints/BP_OverheadWires.BP_OverheadWires_C")
    (bind _asbp_overhead_wires (cast `/Game/Shinkansen/Model/TrainStation/Blueprints/BP_OverheadWires` (`ChildActorComponent.ChildActor` _returnvalue)))
    (`KismetArrayLibrary.Array_Add` (`self.All Child Actors of OverheadPole`) _asbp_overhead_wires))
  ;[1 1 1] Gets start and end of first cable, and sets its position based on the spline
  (for _index_2 (range (+ (`self.Number Of Spline Points`) 1))
    (set `self.Index Loop 2` _index_2)
    (`|ExecutionSequence`
      (:`then_0`
        (`SceneComponent.K2_AttachToComponent` (`/Game/Shinkansen/Model/TrainStation/Blueprints/BP_OverheadWires.Cable1` (`|GetArrayItem` (`self.All Child Actors of OverheadPole`) (`self.Index Loop 2`))) (`/Game/Shinkansen/Model/TrainStation/Blueprints/BP_OverheadWires.Con1` (`|GetArrayItem` (`self.All Child Actors of OverheadPole`) (+ (`self.Index Loop 2`) 1))) "None" "SnapToTarget" "SnapToTarget" "KeepWorld" true))
      (:`then_1`
        ;[1 1 1] Same as above, but for the second cable
        (`SceneComponent.K2_AttachToComponent` (`/Game/Shinkansen/Model/TrainStation/Blueprints/BP_OverheadWires.Cable2` (`|GetArrayItem` (`self.All Child Actors of OverheadPole`) (`self.Index Loop 2`))) (`/Game/Shinkansen/Model/TrainStation/Blueprints/BP_OverheadWires.Con2` (`|GetArrayItem` (`self.All Child Actors of OverheadPole`) (+ (`self.Index Loop 2`) 1))) "None" "SnapToTarget" "SnapToTarget" "KeepWorld" true)))))