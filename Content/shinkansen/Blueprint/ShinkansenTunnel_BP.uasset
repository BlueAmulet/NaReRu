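; Shinkansen tunnel actor that slides along a timeline-driven path, likely to simulate train motion through a tunnel.
; The timeline starts on BeginPlay or the トンネル event, sets the actor's relative location, and destroys it two seconds after finishing.
; A timeline event track spawns the next tunnel at a fixed location while Spawnable is true, forming a self-replicating chain.
; The 消去 event clears Spawnable and destroys the actor.
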(event `トンネル`
  (bind (_direction _starttimeline) (`Timeline|タイムライン_0` :!via `PlayFromStart` :!label _label)
    (:`Update`
      (`self.K2_SetActorRelativeLocation` _starttimeline))
    (:`Finished`
      (`KismetSystemLibrary.Delay` 2.0)
      (`self.K2_DestroyActor`))
    (:`トンネルスポーン`
      (if (`self.Spawnable`)
        (`|SpawnActorFromClass` "ShinkansenTunnel_BP_C" (`KismetMathLibrary.MakeTransform` (130.0 40430.0 -90.0)) "Undefined" "OverrideRootScale" null null)))))

(event `self.ReceiveBeginPlay`
  (goto _label :!via `PlayFromStart`))

(event `消去`
  (set `self.Spawnable` false)
  (`self.K2_DestroyActor`))

(fn `UserConstructionScript`)