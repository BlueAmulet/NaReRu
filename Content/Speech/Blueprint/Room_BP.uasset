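; Room_BP is a seated character in a speech scene, apparently an audience member, that reacts to level settings and looks toward the player.
; Once ChangeLevel_BP reports Input, a randomly delayed loop drives Sit_AnimBP: clapping if flagged, otherwise normal, arms-crossed or bored poses weighted by AnimationLevel.
; The loop also plays a timeline-driven blink morph.
; Tick feeds the look vector from the headset position, falling back to player location without tracking.
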(event `self.ReceiveBeginPlay`
  (bind _returnvalue (`SkeletalMeshComponent.GetAnimInstance` (`self.SkeletalMeshComponent`)))
  ;[1 1 1] アニメーション変更
  (bind _outactors (`GameplayStatics.GetAllActorsOfClass` "/Script/Engine.Actor" :!label _label))
  (for _array_element _outactors
    (bind _aschange_level_bp (cast `/Game/Speech/Blueprint/ChangeLevel_BP` _array_element)) ; ChangeLevel_BPからアニメーション設定を読み込む
    (if (`/Game/Speech/Blueprint/ChangeLevel_BP.Input` _aschange_level_bp)
      (`KismetSystemLibrary.Delay` (`KismetMathLibrary.RandomFloatInRange` 0.0 2.0))
      (bind _outactors_2 (`GameplayStatics.GetAllActorsOfClass` "/Script/Engine.Actor"))
      (for _array_element_2 _outactors_2
        (bind _aschange_level_bp_2 (cast `/Game/Speech/Blueprint/ChangeLevel_BP` _array_element_2)) ; ChangeLevel_BPからアニメーション設定を読み込む
        (if (`/Game/Speech/Blueprint/ChangeLevel_BP.Clap` _aschange_level_bp_2)
          (bind _assit_anim_bp (cast `/Game/Speech/Blueprint/Sit_AnimBP` _returnvalue))
          (set `/Game/Speech/Blueprint/Sit_AnimBP.SitAnimValue` 2 _assit_anim_bp) ; 拍手
          (bind (_direction _blinkcurve) (`Timeline|まばたき` :!label _label_2)
            (:`Update`
              (`SkeletalMeshComponent.SetMorphTarget` (`self.SkeletalMeshComponent`) "Eye_Blink" _blinkcurve true)
              (goto _label)))
          (elif (>= (`/Game/Speech/Blueprint/ChangeLevel_BP.AnimationLevel` _aschange_level_bp_2) (`KismetMathLibrary.RandomInteger` 100))
            (bind _assit_anim_bp_2 (cast `/Game/Speech/Blueprint/Sit_AnimBP` _returnvalue))
            (set `/Game/Speech/Blueprint/Sit_AnimBP.SitAnimValue` 1 _assit_anim_bp_2) ; ノーマル
            (goto _label_2)
            (else
              (bind _assit_anim_bp_3 (cast `/Game/Speech/Blueprint/Sit_AnimBP` _returnvalue))
              (if (== (`KismetMathLibrary.RandomInteger` 2) 1)
                (set `/Game/Speech/Blueprint/Sit_AnimBP.SitAnimValue` 0 _assit_anim_bp_3) ; 腕組
                (goto _label_2)
                (else
                  (set `/Game/Speech/Blueprint/Sit_AnimBP.SitAnimValue` 4 _assit_anim_bp_3) ; 退屈
                  (goto _label_2)))))))
      (else
        (`KismetSystemLibrary.Delay` 1.0)
        (goto _label)))))

(event `self.ReceiveTick`
  (params (DeltaSeconds :type "Float (single-precision)"))
  (bind (_devicerotation _deviceposition) (`HeadMountedDisplayFunctionLibrary.GetOrientationAndPosition`))
  (bind _returnvalue (`GameplayStatics.GetPlayerCharacter` 0))
  (bind _returnvalue_location (`KismetMathLibrary.BreakTransform` (`self.GetTransform` _returnvalue)))
  (bind (_returnvalue_x _returnvalue_y _returnvalue_z) (`KismetMathLibrary.BreakVector` (`KismetMathLibrary.SelectVector` (`KismetMathLibrary.TransformLocation` (`self.GetTransform` _returnvalue) (`KismetMathLibrary.LessLess_VectorRotator` _deviceposition _devicerotation)) _returnvalue_location (`HeadMountedDisplayFunctionLibrary.HasValidTrackingPosition`))))
  ;[1 1 1] 姿勢制御
  (bind _assit_anim_bp (cast `/Game/Speech/Blueprint/Sit_AnimBP` (`SkeletalMeshComponent.GetAnimInstance` (`self.SkeletalMeshComponent`))))
  (set `/Game/Speech/Blueprint/Sit_AnimBP.SitLook` (`KismetMathLibrary.MakeVector` _returnvalue_z _returnvalue_y (* _returnvalue_x -10.0)) _assit_anim_bp)
  (set `/Game/Speech/Blueprint/Sit_AnimBP.SitAlpha` 2.0 _assit_anim_bp))

(fn `UserConstructionScript`)