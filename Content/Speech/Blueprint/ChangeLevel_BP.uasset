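; Keyboard-driven control Blueprint that switches an animation level and triggers applause, apparently for a speech scene.
; Numpad operator keys set AnimationLevel to one of four percentage presets, starting at full on BeginPlay; C sets Clap and plays a hall clap sound at a fixed location.
; Each press raises an Input flag and prints the choice; release clears Input after a delay.
; Clap is never reset here, and nothing here reads these variables.
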(event `self.ReceiveBeginPlay`
  (set `self.AnimationLevel` 100 :!label _label)
  (set `self.Input` true)
  (`KismetSystemLibrary.PrintString` "100%"))

(event `Key|Divide`
  (params (Key :type "Key Structure"))
  (:`Pressed`
    (goto _label))
  (:`Released`
    (`KismetSystemLibrary.Delay` 5.0)
    (set `self.Input` false)))

(event `Key|Multiply`
  (params (Key :type "Key Structure"))
  (:`Pressed`
    (set `self.AnimationLevel` 50)
    (set `self.Input` true)
    (`KismetSystemLibrary.PrintString` "50%"))
  (:`Released`
    (`KismetSystemLibrary.Delay` 5.0)
    (set `self.Input` false)))

(event `Key|Subtract`
  (params (Key :type "Key Structure"))
  (:`Pressed`
    (set `self.AnimationLevel` 20)
    (set `self.Input` true)
    (`KismetSystemLibrary.PrintString` "20%"))
  (:`Released`
    (`KismetSystemLibrary.Delay` 5.0)
    (set `self.Input` false)))

(event `Key|Add`
  (params (Key :type "Key Structure"))
  (:`Pressed`
    (set `self.AnimationLevel` 0)
    (set `self.Input` true)
    (`KismetSystemLibrary.PrintString` "0%"))
  (:`Released`
    (`KismetSystemLibrary.Delay` 5.0)
    (set `self.Input` false)))

(event `Key|C`
  (params (Key :type "Key Structure"))
  (:`Pressed`
    (set `self.Clap` true) ; 拍手
    (set `self.Input` true)
    (`KismetSystemLibrary.PrintString` "拍手")
    (`GameplayStatics.PlaySoundAtLocation` "/Game/Speech/Audio/Clap_Hall.Clap_Hall" (-1395.0 -1508.0 -230.0) (struct) 1.0 1.0 0.0 "/Game/Speech/Audio/SoundAttenuation.SoundAttenuation" null null))
  (:`Released`
    (`KismetSystemLibrary.Delay` 5.0)
    (set `self.Input` false)))

(fn `UserConstructionScript`)