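; Seated audience member for a conference-hall speech scene that switches between clapping, normal, arms-crossed and bored animations.
; From BeginPlay it polls ChangeLevel_BP every second until Input is set, then loops with a short random delay to desynchronize reactions.
; Each pass sets SitAnimValue on Sit_AnimBP: Clap forces applause, otherwise AnimationLevel weights normal against a random choice of arms-crossed or bored.
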(event `self.ReceiveBeginPlay`
  (bind _returnvalue (`SkeletalMeshComponent.GetAnimInstance` (`self.SkeletalMeshComponent`)))
  (bind _outactors (`GameplayStatics.GetAllActorsOfClass` "/Script/Engine.Actor" :!label _label))
  (for _array_element _outactors
    (bind _aschange_level_bp (cast `/Game/Speech/Blueprint/ChangeLevel_BP` _array_element)) ; ChangeLevel_BPからアニメーション設定を読み込む
    (if (`/Game/Speech/Blueprint/ChangeLevel_BP.Input` _aschange_level_bp)
      (`KismetSystemLibrary.Delay` (`KismetMathLibrary.RandomFloatInRange` 0.0 2.0))
      (bind _outactors_2 (`GameplayStatics.GetAllActorsOfClass` "/Script/Engine.Actor"))
      (for _array_element_2 _outactors_2
        (bind _aschange_level_bp_2 (cast `/Game/Speech/Blueprint/ChangeLevel_BP` _array_element_2)) ; ChangeLevel_BPからアニメーション設定を読み込む
        (if (`/Game/Speech/Blueprint/ChangeLevel_BP.Clap` _aschange_level_bp_2)
          (bind _assit_anim_bp (cast `/Game/Speech/Blueprint/Sit_AnimBP` _returnvalue))
          (set `/Game/Speech/Blueprint/Sit_AnimBP.SitAnimValue` 2 _assit_anim_bp) ; 拍手
          (goto _label)
          (elif (>= (`/Game/Speech/Blueprint/ChangeLevel_BP.AnimationLevel` _aschange_level_bp_2) (`KismetMathLibrary.RandomInteger` 100))
            (bind _assit_anim_bp_2 (cast `/Game/Speech/Blueprint/Sit_AnimBP` _returnvalue))
            (set `/Game/Speech/Blueprint/Sit_AnimBP.SitAnimValue` 1 _assit_anim_bp_2) ; ノーマル
            (goto _label)
            (else
              (bind _assit_anim_bp_3 (cast `/Game/Speech/Blueprint/Sit_AnimBP` _returnvalue))
              (if (== (`KismetMathLibrary.RandomInteger` 2) 1)
                (set `/Game/Speech/Blueprint/Sit_AnimBP.SitAnimValue` 0 _assit_anim_bp_3) ; 腕組
                (goto _label)
                (else
                  (set `/Game/Speech/Blueprint/Sit_AnimBP.SitAnimValue` 4 _assit_anim_bp_3) ; 退屈
                  (goto _label)))))))
      (else
        (`KismetSystemLibrary.Delay` 1.0)
        (goto _label)))))

(fn `UserConstructionScript`)