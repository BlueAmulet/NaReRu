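; Elevator system actor that ties an elevator box child actor to the door frames on each floor.
; On BeginPlay it attaches every frame in ArrayDoorFrames to itself, keeping world position and rotation.
; It writes each frame's Z offset from the system's origin into the box's ArrayFloors, indexed by floor number, as the floor heights.
; A separate event sends a floor number to every frame's LED display.
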(event `eventAddDoorFrame`
  (params (doorFrame :type "/Game/Elevator/Model/Elevator/Blueprints/Elevator1/BP_DoorFrame Object Reference (by ref)"))
  ;[1 1 1] Make this door frame a child of the Elevator System
  ; Add the height distance to an array representing the height for each floor
  (`self.K2_AttachToActor` doorFrame self "None" "KeepWorld" "KeepWorld" "KeepRelative" false)
  (bind _asbp_elevator_box (cast `/Game/Elevator/Model/Elevator/Blueprints/Elevator1/BP_Elevator_Box` (`ChildActorComponent.ChildActor` (`self.Elevator_Box`))))
  (`KismetArrayLibrary.Array_Set` (`/Game/Elevator/Model/Elevator/Blueprints/Elevator1/BP_Elevator_Box.arrayFloors` _asbp_elevator_box) (`/Game/Elevator/Model/Elevator/Blueprints/Elevator1/BP_DoorFrame.floorNumber` doorFrame) (.z (- (`self.K2_GetActorLocation` doorFrame) (`self.K2_GetActorLocation`))) true))

(event `SetAllDoorFrames_LEDDisplay`
  (params (floorNumber :type Integer))
  ;[1 1 1] Set the LED displays for ALL floors that are part of this Elevator System
  (for (_array_element _array_index) (`self.arrayDoorFrames`)
    (if (>= _array_index 0)
      (`/Game/Elevator/Model/Elevator/Blueprints/Elevator1/BP_DoorFrame.SetFloorLEDDisplay` _array_element floorNumber))))

(event `self.ReceiveBeginPlay`
  ;[1 1 1] Set up and add each door frame to our Elevator System
  (for _array_element (`self.arrayDoorFrames`)
    (`self.eventAddDoorFrame` _array_element)))

(fn `UserConstructionScript`)