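; Elevator door frame for one floor, with sliding doors, two call buttons, a floor sign and an LED display.
; Opening turns off the call buttons and starts a Tick-checked timer that closes the doors.
; Closing reopens if the player trigger is occupied or a dot-product hit test detects an obstruction.
; Dynamic materials offset atlas UVs to show this floor's number and the elevator's current floor.
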(event `self.ReceiveBeginPlay`
  (bind _floornumber (`self.floorNumber`))
  ;[1 1 1] Initialize Variables and set up Actors
  (bind _asbp_call_button (cast `/Game/Elevator/Model/Elevator/Blueprints/Elevator1/BP_callButton` (`ChildActorComponent.ChildActor` (`self.callButton`))))
  (set `/Game/Elevator/Model/Elevator/Blueprints/Elevator1/BP_callButton.floorNumber` _floornumber _asbp_call_button)
  (bind _asbp_call_button_2 (cast `/Game/Elevator/Model/Elevator/Blueprints/Elevator1/BP_callButton` (`ChildActorComponent.ChildActor` (`self.callButton2`))))
  (set `/Game/Elevator/Model/Elevator/Blueprints/Elevator1/BP_callButton.floorNumber` _floornumber _asbp_call_button_2)
  (set `self.doorSpeed` (/ 2.0 (`self.doorSpeed`)))
  (set `self.rightDoorClosedPos` (`SceneComponent.RelativeLocation` (`self.RightDoor`)))
  (set `self.leftDoorClosedPos` (`SceneComponent.RelativeLocation` (`self.LeftDoor`)))
  (set `self.rightDoorOpenWorldPosition` (`SceneComponent.K2_GetComponentLocation` (`self.RightDoor`)))
  (set `self.leftDoorOpenWorldPosition` (`SceneComponent.K2_GetComponentLocation` (`self.LeftDoor`))))

(event `eventCloseDoors`
  ;[1 1 1] Close Doors
  (if (>= (`KismetArrayLibrary.Array_Length` (`PrimitiveComponent.GetOverlappingActors` (`self.playerTrigger`) null)) 1)
    (`self.eventOpenDoors`)
    (else
      (`GameplayStatics.SpawnSoundAttached` "/Game/Elevator/Model/Elevator/Sounds/DoorClose.DoorClose" (`self.Audio`) "None" (0.0 0.0 0.0) (struct) "KeepRelativeOffset" false 0.2 1.0 0.0 null null)
      (set `self.doorsClosing` true)
      (set `self.closeDoorTime` (+ (`KismetSystemLibrary.GetGameTimeInSeconds`) 10000000000.0))
      (`|ExecutionSequence`
        (:`then_0`
          (`KismetSystemLibrary.MoveComponentTo` (`self.rightDoor`) (`self.rightDoorClosedPos`) (struct) false false (`self.doorSpeed`)))
        (:`then_1`
          (`KismetSystemLibrary.MoveComponentTo` (`self.LeftDoor`) (`self.leftDoorClosedPos`) (struct) false false (`self.doorSpeed`))))
      (set `self.doorsClosing` false))))

(event `eventOpenDoors`
  ;[1 1 1] Open Doors
  (set `self.doorsOpening` true)
  (`GameplayStatics.SpawnSoundAttached` "/Game/Elevator/Model/Elevator/Sounds/doorOpen.doorOpen" (`self.Audio`) "None" (0.0 0.0 0.0) (struct) "KeepRelativeOffset" false 0.2 1.0 0.0 null null)
  (set `self.closeDoorTime` (+ (`KismetSystemLibrary.GetGameTimeInSeconds`) (`self.timetoWaitAtFloors`)))
  (`|ExecutionSequence`
    (:`then_0`
      (`KismetSystemLibrary.MoveComponentTo` (`self.LeftDoor`) (`self.leftDoorOpenPos`) (struct) false false (`self.doorSpeed`))
      ;;[1 1 1] We arrived at our floor --> Turn OFF any call buttons
      (bind _asbp_call_button (cast `/Game/Elevator/Model/Elevator/Blueprints/Elevator1/BP_callButton` (`ChildActorComponent.ChildActor` (`self.callButton`))))
      (`/Game/Elevator/Model/Elevator/Blueprints/Elevator1/BP_callButton.TurnOff` _asbp_call_button)
      (bind _asbp_call_button_2 (cast `/Game/Elevator/Model/Elevator/Blueprints/Elevator1/BP_callButton` (`ChildActorComponent.ChildActor` (`self.callButton2`))))
      (`/Game/Elevator/Model/Elevator/Blueprints/Elevator1/BP_callButton.TurnOff` _asbp_call_button_2))
    (:`then_1`
      (`KismetSystemLibrary.MoveComponentTo` (`self.RightDoor`) (`self.rightDoorOpenPos`) (struct) false false (`self.doorSpeed`))
      (set `self.doorsOpening` false))))

(event `SetFloorLEDDisplay`
  (params (currentFloor :type Integer))
  (bind _returnvalue (- currentFloor 1))
  (bind _material_leddisplay (`self.Material_LEDDisplay`))
  ;[1 1 1] Change the LED Display to show the elevator's current floor
  (`MaterialInstanceDynamic.SetScalarParameterValue` _material_leddisplay "TextureOffset_U" (* (`KismetMathLibrary.Conv_IntToDouble` (`.ReturnValue` (`KismetMathLibrary.FMod` (`KismetMathLibrary.Conv_IntToDouble` _returnvalue) 10.0))) 0.1))
  (`MaterialInstanceDynamic.SetScalarParameterValue` _material_leddisplay "TextureOffset_V" (* (mod _returnvalue 10) 0.1)))

(event `self.ReceiveTick`
  (params (DeltaSeconds :type "Float (single-precision)"))
  ;[1 1 1] Event Tick : Check to see if we should close the doors
  (`|ExecutionSequence`
    (:`then_0`
      (if (<= (`self.closeDoorTime`) (`KismetSystemLibrary.GetGameTimeInSeconds`))
        (`self.eventCloseDoors`)))))

(event `self.LeftDoor.OnComponentHit`
  (params (HitComponent :type "PrimitiveComponent Object Reference") (OtherActor :type "Actor Object Reference") (OtherComp :type "PrimitiveComponent Object Reference") (NormalImpulse :type "Vector Structure") (Hit :type "HitResult Structure (by ref)"))
  (bind _returnvalue (`SceneComponent.K2_GetComponentLocation` (`self.leftDoor`)))
  (bind _returnvalue_2 (`SceneComponent.K2_GetComponentLocation` (`self.rightDoor`)))
  ;[1 1 1] Check for any physics objects preventing the door from closing
  (if (and (`self.doorsClosing`) (or (<= (`KismetMathLibrary.Dot_VectorVector` (`KismetMathLibrary.Normal` (- (`.ImpactPoint` (`GameplayStatics.BreakHitResult` Hit)) _returnvalue)) (`KismetMathLibrary.Normal` (- _returnvalue (`self.leftDoorOpenWorldPosition`)))) -0.7) (<= (`KismetMathLibrary.Dot_VectorVector` (`KismetMathLibrary.Normal` (- (`.ImpactPoint` (`GameplayStatics.BreakHitResult` (stale `self.RightDoor.OnComponentHit` Hit))) _returnvalue_2)) (`KismetMathLibrary.Normal` (- _returnvalue_2 (`self.rightDoorOpenWorldPosition`)))) -0.7)) (not (`self.doorsOpening`))) :!label _label
    (`self.eventOpenDoors`)))

(event `self.RightDoor.OnComponentHit`
  (params (HitComponent :type "PrimitiveComponent Object Reference") (OtherActor :type "Actor Object Reference") (OtherComp :type "PrimitiveComponent Object Reference") (NormalImpulse :type "Vector Structure") (Hit :type "HitResult Structure (by ref)"))
  ;[1 1 1] Check for any physics objects preventing the door from closing
  (goto _label))

(fn `UserConstructionScript`
  (locals (ledFloors :type "MaterialInstanceDynamic Object Reference"))
  (bind _returnvalue (- (`self.floorNumber`) 1))
  (set `self.closeDoorTime` 8.375319268106961e+18)
  ;[1 1 1] Adjust the UVs of the Floor sign material so it matches this Floor Number
  (bind _returnvalue_2 (`PrimitiveComponent.CreateDynamicMaterialInstance` (`self.sm_floorSign`) 0 null "None"))
  (`MaterialInstanceDynamic.SetScalarParameterValue` _returnvalue_2 "TextureOffset_U" (* (mod _returnvalue 9) 0.11))
  (`MaterialInstanceDynamic.SetScalarParameterValue` _returnvalue_2 "TextureOffset_V" (* (`KismetMathLibrary.Conv_IntToDouble` (`.ReturnValue` (`KismetMathLibrary.FMod` (`KismetMathLibrary.Conv_IntToDouble` _returnvalue) 9.0))) 0.1))
  (bind _returnvalue_3 (`PrimitiveComponent.CreateDynamicMaterialInstance` (`self.DoorFrame`) 1 null "None"))
  (set `self.Material_LEDDisplay` _returnvalue_3))